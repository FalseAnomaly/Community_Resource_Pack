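; M3 vehicle for the Z mode that carries extra passengers, acts as a rearm point with unlimited ammo, and force-ends the match when killed.
; Once enough regular seats are filled, users attach to free sockets; Tick turns their view with the hull, and wounds or death detach them to random exit points.
; It also kills soldiers on hard front or rear impacts, syncs headlights to engine state, and has a non-shipping debug camera.
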(event OnComponentHit(VehicleMesh)
  (params (HitComponent :type Primitive%20Component%20Object%20Reference) (OtherActor :type Actor%20Object%20Reference) (OtherComp :type Primitive%20Component%20Object%20Reference) (NormalImpulse :type Vector :default "0, 0, 0") (Hit :type Hit%20Result%20Structure%20%28by%20ref%29))
  (bind _returnvalue (Math|Float|MakeLiteralFloat 0.86))
  (bind _vehiclemesh (Variables|Default|GetVehicleMesh))
  (bind _returnvalue_2 (Math|Vector|GetForwardVector _vehiclemesh))
  (Networking|SwitchHasAuthority
    (:Authority
      (bind _aspssoldier (Utilities|Casting|CastToPSSoldier OtherActor))
      (if (Math|Boolean|ANDBoolean (> (CallFunction|GetOccupiedSeatsCount) 0) (>= (Math|Vector|VectorLengthSquared NormalImpulse) (Variables|Default|GetImpactKillImpulseSq)) (or (>= (Math|Vector|DotProduct NormalImpulse _returnvalue_2) _returnvalue) (>= (Math|Vector|DotProduct NormalImpulse (Math|Vector|NegateVector _returnvalue_2)) _returnvalue)))
        (Game|Damage|ApplyDamage _aspssoldier 114514.0 (Pawn|GetController) self "/Game/Gameplay/DamageTypes/BP_Melee.BP_Melee_C")))))

(event Custom|RepDoDamageFX
  (params (Location :type Vector))
  (Networking|CanExecuteCosmeticEvents
    (:True
      (Audio|SpawnSoundatLocation "/Game/Audio/Impacts/Bullethits/Metal_thick/Metal_thick_cue.Metal_thick_cue" Location "0, 0, 0" 1.0 1.0 0.0 0 0)
      (Effects|SpawnEmitteratLocation "/Game/Particles/Impacts/Bullethits/50cal/Vehicle/Bhit_Metal_50cal.Bhit_Metal_50cal" Location))))

(event Custom|OnFreePassengerDied
  (params (DeadSoldier :type PS%20Soldier%20Object%20Reference) (Killer :type Pawn%20Object%20Reference) (DamageCauser :type Actor%20Object%20Reference) (bPointDamage :type Boolean))
  (CallFunction|DetachSoldierfromSocket DeadSoldier))

(event Custom|OnFreePassangerWounded
  (params (KillingDamage :type Float%20%28single-precision%29) (DamageEvent :type Damage%20Event%20Structure) (Killer :type Controller%20Object%20Reference) (DamageCauser :type Actor%20Object%20Reference) (WoundedSoldat :type BP%20PS%20Mutable%20Soldier%20Object%20Reference))
  (CallFunction|DetachSoldierfromSocket WoundedSoldat))

(event EventOnEngineStatusChanged
  (bind _bisengineactive (Variables|Default|GetbIsEngineActive))
  (Networking|CanExecuteCosmeticEvents
    (:True
      (Rendering|SetVisibility (Variables|Default|GetSpotLight) _bisengineactive true)
      (Rendering|Material|SetScalarParameterValue (Variables|Default|GetHeadlightDynamicMaterial) "HeadlightStrength" (select _bisengineactive 1.0 0.0) :!class /Script/Engine.MaterialInstanceDynamic))))

(event EventServeronUsed
  (params (User :type Controller%20Object%20Reference))
  (if (CallFunction|IsAlreadyAttached User)
    (CallFunction|DetachSoldierfromSocket (Pawn|GetControlledPawn User))
    (elif (>= (CallFunction|GetOccupiedSeatsCount) (Variables|Default|GetMinPlayersInVehicleBeforeAttaching))
      (if (CallFunction|IsFreeSeatsFull)
        (bind _asbp_ps_player_controller (Utilities|Casting|CastToBP_PS_PlayerController User))
        (Default|ClientNotification _asbp_ps_player_controller "Vehicle Is full" "Error")
        (else
          (CallFunction|SeatSoldiertoSocket User)))
      (else
        (|CallParentFunction User)))))

(event EventTick
  (params (DeltaSeconds :type Float%20%28single-precision%29))
  (|CallParentFunction DeltaSeconds)
  (Variables|Default|SetDeltaRotation (Math|Rotator|CombineRotators (Transformation|GetActorRotation) (Class|KismetMathLibrary|NegateRotator (Variables|Default|GetLastRotation))))
  (for _array_element (Variables|Default|GetSeatedSoldier)
    (Utilities|IsValid (Pawn|GetController _array_element)
      (:Is%20Valid
        (if (Pawn|IsLocallyControlled _array_element)
          (Pawn|SetControlRotation (Pawn|GetController _array_element) (Math|Rotator|CombineRotators (Math|Rotator|MakeRotator 0.0 (.Pitch (Math|Rotator|BreakRotator (Pawn|GetControlRotation _array_element :!class /Script/Engine.Pawn))) (.Yaw (Math|Rotator|BreakRotator (Pawn|GetControlRotation _array_element :!class /Script/Engine.Pawn)))) (Math|Rotator|MakeRotator 0.0 0.0 (.Yaw (Math|Rotator|BreakRotator (Variables|Default|GetDeltaRotation))))))
          (Transformation|SetActorRotation _array_element (Math|Rotator|MakeRotator 0.0 0.0 (.Yaw (Math|Rotator|BreakRotator (Transformation|GetActorRotation _array_element)))) true)))))
  (Variables|Default|SetLastRotation (Transformation|GetActorRotation)))

(event EventBeginPlay
  (bind _bisengineactive (Variables|Default|GetbIsEngineActive))
  (Class|PrimitiveComponent|SetNotifyRigidBodyCollision (Variables|Default|GetVehicleMesh) true)
  (Networking|CanExecuteCosmeticEvents
    (:True
      (Rendering|SetVisibility (Variables|Default|GetSpotLight) _bisengineactive true)
      (Rendering|Material|SetScalarParameterValue (Variables|Default|GetHeadlightDynamicMaterial) "HeadlightStrength" (select _bisengineactive 1.0 0.0) :!class /Script/Engine.MaterialInstanceDynamic))))

(event EventOnVehicleKilled
  (params (Vehicle :type SQ%20Vehicle%20Object%20Reference) (Killer :type Controller%20Object%20Reference) (DamageCauser :type Actor%20Object%20Reference))
  (bind _asbp_game_mode (Utilities|Casting|CastToBP_GameMode (Game|GetGameMode)))
  (Default|ForceEndMatch _asbp_game_mode 1)
  (Utilities|FlowControl|Delay 1.0)
  (Actor|DestroyActor))

(event Input|ActionEvents|InputActionToggleView
  (params (Key :type Key%20Structure))
  (bind _activecamera (Variables|Default|GetActiveCamera))
  (bind _externalcamera (Variables|Default|GetExternalCamera))
  ;[1 1 1] Third Person Debug Camera
  (:Pressed
    (if (not (Class|SQBlueprintLibrary|IsShippingBuild))
      (if (Components|Activation|IsActive (Variables|Default|GetActiveCamera))
        (Components|Activation|Deactivate _activecamera)
        (Components|Activation|Activate _externalcamera false)
        (else
          (Components|Activation|Activate _activecamera false)
          (Components|Activation|Deactivate _externalcamera))))))

(event Input|MouseEvents|MouseX
  (params (AxisValue :type Float%20%28single-precision%29))
  ;[1 1 1] Third Person Debug Camera
  (if (Components|Activation|IsActive (Variables|Default|GetExternalCamera))
    (Transformation|AddLocalRotation (Variables|Default|GetSpringArm) (Math|Rotator|MakeRotator 0.0 0.0 AxisValue) false false)))

(event Input|MouseEvents|MouseY
  (params (AxisValue :type Float%20%28single-precision%29))
  ;[1 1 1] Third Person Debug Camera
  (if (Components|Activation|IsActive (Variables|Default|GetExternalCamera))
    (Transformation|AddLocalRotation (Variables|Default|GetSpringArm) (Math|Rotator|MakeRotator 0.0 AxisValue 0.0) false false)))

(event Input|MouseEvents|MouseWheelUp
  (params (Key :type Key%20Structure))
  (bind _springarm (Variables|Default|GetSpringArm))
  ;[1 1 1] Third Person Debug Camera
  (:Pressed
    (if (Components|Activation|IsActive (Variables|Default|GetExternalCamera))
      (Variables|/Script/Engine.SpringArmComponent|SetTargetArmLength _springarm (Math|Float|Max(Float) (- (Variables|/Script/Engine.SpringArmComponent|GetTargetArmLength _springarm) 25.0) 0.0)))))

(event Input|MouseEvents|MouseWheelDown
  (params (Key :type Key%20Structure))
  (bind _springarm (Variables|Default|GetSpringArm))
  ;[1 1 1] Third Person Debug Camera
  (:Pressed
    (if (Components|Activation|IsActive (Variables|Default|GetExternalCamera))
      (Variables|/Script/Engine.SpringArmComponent|SetTargetArmLength _springarm (+ (Variables|/Script/Engine.SpringArmComponent|GetTargetArmLength _springarm) 25.0)))))

(fn ConstructionScript
  (|CallParentFunction)
  (bind _returnvalue (Rendering|Material|CreateDynamicMaterialInstance (Variables|Default|GetVehicleMesh) 2 0 "None" :!class /Script/Engine.PrimitiveComponent))
  (Variables|Default|SetHeadlightDynamicMaterial _returnvalue)
  (Variables|Default|SetExitPoints (Utilities|Array|MakeArray (Variables|Default|GetSQVehicleExitPoint) (Variables|Default|GetSQVehicleExitPoint1) (Variables|Default|GetSQVehicleExitPoint2) (Variables|Default|GetSQVehicleExitPoint3)))
  (Variables|/Game/PostScriptum/Gameplay/BP_VehicleMSPComponent.BP_VehicleMSPComponent_C|SetSpawnLocation (Variables|Default|GetBP_VehicleMSPComponent) (Variables|Default|GetSpawnpoint_Location)))

(fn GetOccupiedSeatsCount
  (for _array_element (Variables|Default|GetVehicleSeats)
    (Utilities|IsValid (Variables|/Script/Squad.SQVehicleSeatComponent|GetSeatedPlayer _array_element)
      (:Is%20Valid
        (Math|Integer|IncrementInt (LocalVariables|GetNumOccupiedSeats)))))
  (return (LocalVariables|GetNumOccupiedSeats)))

(fn SeatSoldiertoSocket
  (params (PlayerController :type Controller%20Object%20Reference))
  (bind _asbp_ps_mutable_soldier (Utilities|Casting|CastToBP_PS_MutableSoldier (Pawn|GetControlledPawn PlayerController)))
  (bind _keys (Utilities|Map|Keys (Variables|Default|GetAttachedSeatPlayers)))
  (bind _array_element (Utilities|Array|ForEachLoopwithBreak _keys :!label _label)
    (:LoopBody
      (bind _bplayerseated (CallFunction|TrySeatingPlayer _array_element _asbp_ps_mutable_soldier))
      (LocalVariables|SetbPlayerSeated _bplayerseated)
      (if (LocalVariables|GetbPlayerSeated)
        (EventDispatchers|BindEventtoOnSoldierDied _asbp_ps_mutable_soldier (EventDispatchers|CreateEvent :!event Custom|OnFreePassengerDied))
        (EventDispatchers|BindEventtoOnSoldierWounded _asbp_ps_mutable_soldier (EventDispatchers|CreateEvent :!event Custom|OnFreePassangerWounded))
        (goto _label Break)))
    (:Completed
      (if (LocalVariables|GetbPlayerSeated)
        (Utilities|Array|AddUnique (Variables|Default|GetSeatedSoldier) _asbp_ps_mutable_soldier)))))

(fn TrySeatingPlayer
  (params (SocketName :type Name%20%28by%20ref%29) (SoldierToSeat :type BP%20PS%20Mutable%20Soldier%20Object%20Reference))
  (bind _attachedseatplayers (Variables|Default|GetAttachedSeatPlayers))
  (bind (_value _returnvalue) (Utilities|Map|Find _attachedseatplayers SocketName))
  (if _returnvalue
    (if (Utilities|IsValid _value)
      (return false)
      (else
        _)))
  (Transformation|AttachComponentToComponent (Variables|/Script/Engine.Character|GetCapsuleComponent SoldierToSeat) (Variables|Default|GetVehicleMesh) SocketName "SnapToTarget" "KeepWorld" "KeepWorld" false)
  (Utilities|Map|Add (Variables|Default|GetAttachedSeatPlayers) SocketName SoldierToSeat)
  (Default|AddBuffClient SoldierToSeat "NoBipod" -1.0)
  (bind _asbp_ps_soldier_z (Utilities|Casting|CastToBP_PS_Soldier_Z SoldierToSeat))
  (Variables|/Community_Resource_Pack/Soldiers/Z/BP_PS_Soldier_Z.BP_PS_Soldier_Z_C|SetAttachedToVehicle _asbp_ps_soldier_z self)
  (return true))

(fn IsAlreadyAttached
  (params (Player :type Controller%20Object%20Reference))
  (for _array_element (Variables|Default|GetSeatedSoldier)
    (if (== (Pawn|GetController _array_element) Player)
      (return true)))
  (return false))

(fn DetachSoldierfromSocket
  (params (Pawn :type Pawn%20Object%20Reference))
  (bind _attachedseatplayers (Variables|Default|GetAttachedSeatPlayers))
  (bind _exitpoints (Variables|Default|GetExitPoints))
  (bind _asbp_ps_mutable_soldier (Utilities|Casting|CastToBP_PS_MutableSoldier Pawn))
  (bind _keys (Utilities|Map|Keys _attachedseatplayers))
  (bind _array_element (Utilities|Array|ForEachLoopwithBreak _keys :!label _label)
    (:LoopBody
      (if (== (.Value (Utilities|Map|Find _attachedseatplayers _array_element)) _asbp_ps_mutable_soldier)
        (Utilities|Map|Add (Variables|Default|GetAttachedSeatPlayers) _array_element 0)
        (Utilities|Array|RemoveItem (Variables|Default|GetSeatedSoldier) _asbp_ps_mutable_soldier)
        (Transformation|DetachFromActor _asbp_ps_mutable_soldier "KeepWorld" "KeepWorld" "KeepWorld")
        (Default|RemoveBuffClient _asbp_ps_mutable_soldier "NoBipod")
        (bind _asbp_ps_soldier_z (Utilities|Casting|CastToBP_PS_Soldier_Z _asbp_ps_mutable_soldier))
        (Variables|/Community_Resource_Pack/Soldiers/Z/BP_PS_Soldier_Z.BP_PS_Soldier_Z_C|SetAttachedToVehicle _asbp_ps_soldier_z 0)
        (EventDispatchers|UnbindEventfromOnSoldierDied _asbp_ps_mutable_soldier (EventDispatchers|CreateEvent :!event Custom|OnFreePassengerDied))
        (EventDispatchers|UnbindEventfromOnSoldierWounded _asbp_ps_mutable_soldier (EventDispatchers|CreateEvent :!event Custom|OnFreePassangerWounded))
        (Transformation|Teleport _asbp_ps_mutable_soldier (Transformation|GetWorldLocation (Utilities|Array|Get(acopy) _exitpoints (Math|Random|RandomIntegerinRange 0 (Utilities|Array|LastIndex _exitpoints)))) (Math|Rotator|MakeRotator 0.0 0.0 (.Yaw (Math|Rotator|BreakRotator (Transformation|GetActorRotation _asbp_ps_mutable_soldier)))))
        (goto _label Break)))))

(fn GetRearmType
  (return "Vehicle"))

(fn CanRearmPawn
  (params (Rearmer :type Pawn%20Object%20Reference))
  (bind _playerstate (Variables|/Script/Engine.Pawn|GetPlayerState Rearmer))
  (bind _playerrearmtimes (Variables|Default|GetPlayerRearmTimes))
  (bind (_value _returnvalue) (Utilities|Map|Find _playerrearmtimes _playerstate))
  (if _returnvalue
    (return (> (- (Utilities|Time|GetTimeSeconds) _value) (Variables|Default|GetRearmCooldown)))
    (else
      (return true))))

(fn ConsumeAmmo
  (params (AmmoRequired :type Float%20%28single-precision%29))
  (return true))

(fn GetAmmo
  (return 1e+04))

(fn CanRearmWeapon
  (params (Weapon :type SQ%20Equipable%20Item%20Object%20Reference))
  (return true))

(fn UnbindEventtoAmmoUpdated
  (params (Delegate :type Delegate%20%28by%20ref%29))
  (return false))

(fn GetRearmSuccessString
  (return "Re-armed successfully"))

(fn GetRearmNoAmmoString
  (return ""))

(fn BindEventtoAmmoUpdated
  (params (Delegate :type Delegate%20%28by%20ref%29))
  (return false))

(fn CanRearmPlayer
  (params (PlayerToRearm :type Pawn%20Object%20Reference))
  (bind _returnvalue (Utilities|Time|GetTimeSeconds))
  (return (Class|SQRearmSource|CanRearmPawn PlayerToRearm) (- (Variables|Default|GetRearmCooldown) (- _returnvalue (.Value (Utilities|Map|Find (Variables|Default|GetPlayerRearmTimes) (Variables|/Script/Engine.Pawn|GetPlayerState PlayerToRearm))))) _returnvalue))

(fn IsFreeSeatsFull
  (bind _values (Utilities|Map|Values (Variables|Default|GetAttachedSeatPlayers)))
  (for _array_element _values
    (Utilities|IsValid _array_element
      (:Is%20Not%20Valid
        (return false))))
  (return true))

(fn DoDamageFX
  (params (Location :type Vector))
  (Audio|SpawnSoundatLocation "/Game/Audio/Impacts/Bullethits/Metal_thick/Metal_thick_cue.Metal_thick_cue" Location "0, 0, 0" 1.0 1.0 0.0 0 0)
  (Effects|SpawnEmitteratLocation "/Game/Particles/Impacts/Bullethits/50cal/Vehicle/Bhit_Metal_50cal.Bhit_Metal_50cal" Location))

(fn GetLoadActor
  (bind _asbp_objective_load_z (Utilities|Casting|CastToBP_ObjectiveLoad_Z (Variables|/Script/Engine.ChildActorComponent|GetChildActor (Variables|Default|GetChildActor)))
    (:then
      (return _asbp_objective_load_z))
    (:CastFailed
      (return 0))))
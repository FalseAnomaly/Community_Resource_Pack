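; A vehicle action that offloads supplies from a ground vehicle at a bomb site.
; On the server, DoAction looks for an overlapping BP_BombSpawner_Z and calls TryActivating on the first one with the player's controller.
; If none overlaps, the player gets an out-of-range toast.
; An "already offloaded" toast exists in the graph but is not wired up.
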(event EventDoAction
  (params (User :type Player%20Controller%20Object%20Reference) (Context :type Object%20Object%20Reference))
  (bind _aspsplayer_controller (Utilities|Casting|CastToPSPlayerController User))
  (bind _assqground_vehicle (Utilities|Casting|CastToSQGroundVehicle Context))
  (if (Ability|HasAuthority _assqground_vehicle)
    (if (Utilities|Array|IsValidIndex (Collision|GetOverlappingActors _assqground_vehicle "/Community_Resource_Pack/Blueprints/Z/BP_BombSpawner_Z.BP_BombSpawner_Z_C" :!class /Script/Engine.Actor))
      (bind _asbp_bomb_spawner_z (Utilities|Casting|CastToBP_BombSpawner_Z (Utilities|Array|Get(acopy) (Collision|GetOverlappingActors _assqground_vehicle "/Community_Resource_Pack/Blueprints/Z/BP_BombSpawner_Z.BP_BombSpawner_Z_C" :!class /Script/Engine.Actor))))
      (Default|TryActivating _asbp_bomb_spawner_z _aspsplayer_controller)
      (else
        (Class|SQPlayerController|ClientShowToast _aspsplayer_controller (Utilities|Text|MakeLiteralText "Bomb site is out of range") 5.0)))))
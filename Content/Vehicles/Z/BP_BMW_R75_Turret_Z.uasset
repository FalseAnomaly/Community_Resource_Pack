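; Player-controlled weapon turret for the BMW R75 vehicle, handling aim, firing and focus zoom.
; Turn and LookUp drive separate yaw and pitch movement components, registered at construction and gated on weapon input being enabled.
; Fire uses the vehicle inventory's current weapon, while Focus narrows camera FOV to two-thirds of the user setting.
; Overrides supply gun and camera attach points; soldier attachment searches vehicle mesh children for BP_NullComponent, with leftover debug printing.
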(event Input|ActionEvents|InputActionFocus
  (params (Key :type Key%20Structure))
  (bind _returnvalue (Class|SQBlueprintLibrary|GetSquadGameUserSettings))
  (bind _fov (Variables|/Script/Squad.SQGameUserSettings|GetFOV _returnvalue))
  ;[1 1 1] Focus FOV shift
  (:Pressed
    (Camera|SetFieldOfView (Variables|Default|GetCamera) (* 0.666 _fov)))
  (:Released
    (Camera|SetFieldOfView (Variables|Default|GetCamera) _fov)))

(event Input|ActionEvents|InputActionFire
  (params (Key :type Key%20Structure))
  (bind _returnvalue (Class|SQVehicleSeat|GetVehicleInventory))
  (bind _currentweapon (Variables|/Script/Squad.SQPawnInventoryComponent|GetCurrentWeapon _returnvalue))
  (:Pressed
    (Class|SQEquipableItem|BeginUse _currentweapon))
  (:Released
    (Class|SQEquipableItem|EndUse _currentweapon)))

(event Input|AxisEvents|InputAxisTurn
  (params (AxisValue :type Float%20%28single-precision%29))
  (bind _returnvalue (Class|SQVehicleTurret|IsCurrentWeaponInputEnabled))
  (if _returnvalue
    (Class|SQRotatingMovementComponent|AddRotationInput (Variables|Default|GetYawMovementComponent) (Math|Rotator|MakeRotator 0.0 0.0 AxisValue))))

(event Input|AxisEvents|InputAxisLookUp
  (params (AxisValue :type Float%20%28single-precision%29))
  (bind _returnvalue (Class|SQVehicleTurret|IsCurrentWeaponInputEnabled))
  (if _returnvalue
    (Class|SQRotatingMovementComponent|AddRotationInput (Variables|Default|GetPitchMovementComponent) (Math|Rotator|MakeRotator 0.0 AxisValue 0.0))))

(fn ConstructionScript
  (|CallParentFunction)
  (Utilities|FlowControl|Sequence
    (:then_0
      (Variables|/Script/Squad.SQRotatingMovementComponent|SetUpdatedComponent (Variables|Default|GetYawMovementComponent) (Variables|Default|GetDefaultSceneRoot))
      (Variables|/Script/Squad.SQRotatingMovementComponent|SetUpdatedComponent (Variables|Default|GetPitchMovementComponent) (Variables|Default|GetTurret_SkeletalMesh))
      (Class|SQMovementComponentManager|RegisterComponent (Variables|Default|GetMovementComponentManager) (Variables|Default|GetYawMovementComponent))
      (Class|SQMovementComponentManager|RegisterComponent (Variables|Default|GetMovementComponentManager) (Variables|Default|GetPitchMovementComponent)))
    (:then_1
      (Class|SQFreeLookComponent|SetFreeLookCamera (Variables|Default|GetFreeLookComponent) (Variables|Default|GetCamera)))))

(fn Get3PAttachComponent
  (return (Variables|Default|GetGunAttachPoint)))

(fn Get1PAttachComponent
  (return (Variables|Default|GetGunAttachPoint)))

(fn GetMasterPoseComponent
  (return 0))

(fn GetWeaponAttachComponent
  (return (Variables|Default|GetGunAttachPoint)))

(fn GetDefaultCameraLocationComponent
  (return (Variables|Default|GetDefaultCameraPosition)))

(fn GetADSCameraLocationComponent
  (return (Variables|Default|GetADSCameraPosition)))

(fn IsSoldierAlive
  (bind _currentweapon (Variables|/Script/Squad.SQPawnInventoryComponent|GetCurrentWeapon (Variables|Default|GetSQVehicleInventory))
    (:then
      (bind _assqvehicle_weapon (Utilities|Casting|CastToSQVehicleWeapon _currentweapon)
        (:then
          (Utilities|IsValid (Class|SQVehicleWeapon|GetSoldier _assqvehicle_weapon)
            (:Is%20Valid
              (return (Class|SQSoldier|IsAlive (Class|SQVehicleWeapon|GetSoldier _assqvehicle_weapon))))
            (:Is%20Not%20Valid
              (return false))))
        (:CastFailed
          (return false))))
    (:else
      (return false))))

(fn GetSoldierAttachComponent
  (bind _returnvalue (Class|SQVehicleSeat|GetVehicle))
  (bind _vehiclemesh (Variables|/Script/Squad.SQVehicle|GetVehicleMesh _returnvalue))
  (bind _children (Components|GetChildrenComponents _vehiclemesh false))
  (bind _index (Utilities|FlowControl|ForLoopwithBreak 0 (- (Class|SceneComponent|GetNumChildrenComponents _vehiclemesh) 1) :!label _label)
    (:LoopBody
      (Development|PrintString (Class|KismetSystemLibrary|GetPathName (Utilities|Array|Get(acopy) _children _index)) true true "(R=0.000000,G=0.660000,B=1.000000,A=1.000000)" 3e+01)
      (Utilities|Casting|CastToBP_NullComponent (Utilities|Array|Get(acopy) _children _index))
      (LocalVariables|SetTemp _index)
      (goto _label Break))
    (:Completed
      (return (Utilities|Array|Get(acopy) _children (LocalVariables|GetTemp))))))
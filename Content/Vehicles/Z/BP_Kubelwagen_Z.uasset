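; Vehicle Blueprint for the Kubelwagen (Z variant) that ties its headlights to the engine state.
; The construction script creates a dynamic material instance on one element of the vehicle mesh for the headlight glow.
; On BeginPlay and whenever engine status changes, both spotlights and the material's HeadlightStrength parameter switch on or off with IsEngineActive.
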(event EventOnEngineStatusChanged
  (bind _bisengineactive (Variables|Default|GetbIsEngineActive))
  (Rendering|SetVisibility (Variables|Default|GetSpotLight) _bisengineactive true)
  (Rendering|Material|SetScalarParameterValue (Variables|Default|GetHeadlightDynamicMaterial) "HeadlightStrength" (select _bisengineactive 1.0 0.0) :!class /Script/Engine.MaterialInstanceDynamic))

(event Collision|EventActorBeginOverlap
  (params (OtherActor :type Actor%20Object%20Reference))
  (|CallParentFunction OtherActor) ; This node is disabled and will not be called.\nDrag off pins to build functionality.
)

(event EventTick
  (params (DeltaSeconds :type Float%20%28single-precision%29))
  (|CallParentFunction DeltaSeconds) ; This node is disabled and will not be called.\nDrag off pins to build functionality.
)

(event EventBeginPlay
  (bind _bisengineactive (Variables|Default|GetbIsEngineActive))
  (|CallParentFunction)
  (Rendering|SetVisibility (Variables|Default|GetSpotLight) _bisengineactive true)
  (Rendering|Material|SetScalarParameterValue (Variables|Default|GetHeadlightDynamicMaterial) "HeadlightStrength" (select _bisengineactive 1.0 0.0) :!class /Script/Engine.MaterialInstanceDynamic))

(fn ConstructionScript
  (|CallParentFunction)
  (bind _returnvalue (Rendering|Material|CreateDynamicMaterialInstance (Variables|Default|GetVehicleMesh) 2 0 "None" :!class /Script/Engine.PrimitiveComponent))
  (Variables|Default|SetHeadlightDynamicMaterial _returnvalue))
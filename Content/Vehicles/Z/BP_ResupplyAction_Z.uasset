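; Resupply action that lets a soldier rearm from an M3_Z vehicle, subject to a per-player wait time.
; CreateResupplyRequest walks every inventory group and requests a full refill, using max mags for weapons and max item count for other items.
; When the vehicle's CanRearmPlayer check passes, the server rearm runs and the player's time is recorded on the vehicle; otherwise a toast shows the remaining wait.
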(event EventDoAction
  (params (User :type Player%20Controller%20Object%20Reference) (Context :type Object%20Object%20Reference))
  (bind _asbp_player_controller (Utilities|Casting|CastToBP_PlayerController User))
  (bind _assqsoldier (Utilities|Casting|CastToSQSoldier (Pawn|GetControlledPawn _asbp_player_controller)))
  (bind _request (CallFunction|CreateResupplyRequest _assqsoldier))
  (bind _assqrearm_source (Utilities|Casting|CastToSQRearmSource Context))
  (bind _asbp_m3_z (Utilities|Casting|CastToBP_M3_Z Context))
  (if (.bCanRearm (Default|CanRearmPlayer _asbp_m3_z (Pawn|GetControlledPawn _asbp_player_controller)))
    (Class|SQPlayerController|BPServerRearmWeapons _asbp_player_controller _assqrearm_source _request)
    (Utilities|Map|Add (Variables|/Community_Resource_Pack/Vehicles/Z/BP_M3_Z.BP_M3_Z_C|GetPlayerRearmTimes _asbp_m3_z) (Variables|/Script/Engine.Pawn|GetPlayerState (Pawn|GetControlledPawn _asbp_player_controller)) (.CurrentTimeSeconds (Default|CanRearmPlayer _asbp_m3_z (Pawn|GetControlledPawn _asbp_player_controller))))
    (else
      (Class|SQPlayerController|ClientShowToast _asbp_player_controller (Utilities|Text|ToText(String) (Utilities|String|Append "Please wait for " (Utilities|String|LeftChop (Class|KismetStringLibrary|TimeSecondstoString (.TimeToWait (Default|CanRearmPlayer _asbp_m3_z (Pawn|GetControlledPawn _asbp_player_controller)))) 3) " Seconds before resupplying again")) 5.0))))

(fn CreateResupplyRequest
  (params (Soldier :type SQ%20Soldier%20Object%20Reference))
  (bind _rearmrequest (LocalVariables|GetRearmRequest))
  (for _array_element (Class|SQPawnInventoryComponent|GetInventoryItemGroups (Class|SQSoldier|GetInventory Soldier))
    (for _array_element_2 (.weapons _array_element)
      (bind _assqweapon (Utilities|Casting|CastToSQWeapon _array_element_2)
        (:then
          (Utilities|Array|Add _rearmrequest (Utilities|Struct|MakeSQRearmWeaponRequest _array_element_2 (.MaxMags (Utilities|Struct|BreakSQWeaponData (Variables|/Script/Squad.SQWeapon|GetWeaponConfig _assqweapon))))))
        (:CastFailed
          (Utilities|Array|Add _rearmrequest (Utilities|Struct|MakeSQRearmWeaponRequest _array_element_2 (Variables|/Script/Squad.SQEquipableItem|GetMaxItemCount _array_element_2)))))))
  (return (LocalVariables|GetRearmRequest)))
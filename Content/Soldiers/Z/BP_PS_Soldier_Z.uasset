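; Soldier pawn for a zombie mode, playable as survivor or zombie, reporting deaths to the player state.
; Zombify swaps in gore materials, local HUD and post-process, and retunes health, jumping and movement.
; Damage builds a decaying ZombieCharge whose OnRep slows zombie movement and, on the server, stops bleeding or regenerates health after a damage-free delay.
; Wounded zombies, and survivors wounded by zombies, die outright; GiveZombieRole supplies the melee loadout.
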(event Custom|SpawnRisingSoul
  (bind _self self)
  (Networking|CanExecuteCosmeticEvents
    (:True
      (Game|SpawnActorfromClass "/Community_Resource_Pack/Blueprints/Z/BP_GhostSoldat_Soul_Lift_Z.BP_GhostSoldat_Soul_Lift_Z_C" (Transformation|GetActorTransform) "AlwaysSpawn" _self _self))))

(event Custom|Zombify
  (params (bSound :type Boolean))
  (bind _returnvalue (Math|Float|MakeLiteralFloat 1.1))
  (bind _returnvalue_2 (Math|Float|MakeLiteralFloat 0.36))
  (bind _soldiermovement (Variables|Default|GetSoldierMovement))
  (bind _maxwalkspeed (Variables|/Script/Engine.CharacterMovementComponent|GetMaxWalkSpeed _soldiermovement))
  (Variables|Default|SetbIsZombie true)
  (Variables|Default|SetbIgnoreTeamDamage true)
  (Utilities|FlowControl|Sequence
    (:then_0
      (CallFunction|GorifyMesh))
    (:then_1
      (Variables|Default|SetSuppressionStaminaRegenMultiplierPenalty 1.0)
      (Variables|Default|SetMaximumSafeFallingSpeed 999999.0))
    (:then_2
      (if (Pawn|IsLocallyControlled)
        (Variables|/Script/Engine.PostProcessComponent|SetbEnabled (Variables|Default|GetPostProcess) true)
        (bind _returnvalue_3 (UserInterface|CreateWidget "/Community_Resource_Pack/UI/UMG_ZombieNotification_Z.UMG_ZombieNotification_Z_C"))
        (bind _returnvalue_4 (UserInterface|CreateWidget "/Community_Resource_Pack/UI/UMG_ZombieHud_Z.UMG_ZombieHud_Z_C" (Game|GetPlayerController 0)))
        (Variables|Default|SetzombieHud _returnvalue_4)
        (UserInterface|Viewport|AddtoViewport _returnvalue_3 0))
      (if bSound
        (bind _returnvalue_5 (Audio|SpawnSoundAttached "/Game/PostScriptum/Gameplay/Halloween/Zombie/Desert_Heat_Cue.Desert_Heat_Cue" (Variables|Character|GetMesh) "None" "0, 0, 0" "0, 0, 0" "SnapToTarget" false 1.0 1.0 0.0 "/Game/PostScriptum/Gameplay/Halloween/Zombie/ZombieMusicAttenuation.ZombieMusicAttenuation" 0))
        (Variables|Default|SetHorrorSound _returnvalue_5)))
    (:then_3
      (Utilities|FlowControl|Delay 1.0)
      (Variables|Default|SetKillDamageThreshold 5e+02)
      (Variables|Default|SetHealthHurtMovementThreshold 0.0)
      (Networking|SwitchHasAuthority
        (:Authority
          (Class|SQSoldier|Heal (Math|Conversions|ToFloat(Integer) (Variables|Default|GetMaxZombieHealth)))
          (Utilities|Time|SetTimerbyEvent (delegate Custom|ZombieLoop) 1.0 true)
          (Variables|Default|SetLastDamageTime 0.0))))
    (:then_4
      (Variables|/Script/Squad.SQSoldierMovement|SetbStaminaLimitsJumping _soldiermovement true)
      (Variables|/Script/Squad.SQSoldierMovement|SetbJumpingUsesStamina _soldiermovement true)
      (Variables|/Script/Squad.SQSoldierMovement|SetStaminaLossPerJump _soldiermovement 15.0)
      (Variables|/Script/Engine.CharacterMovementComponent|SetJumpZVelocity _soldiermovement 6e+02)
      (Variables|Default|SetDefaultWalkSpeed (* _maxwalkspeed _returnvalue_2))
      (bind _output_get (Variables|Default|SetDefaultProneSpeed (* (Variables|/Script/Squad.SQSoldierMovement|GetMaxWalkSpeedProne _soldiermovement) _returnvalue_2)))
      (bind _output_get_2 (Variables|Default|SetdefaultCrouchSpeed (* _returnvalue_2 (Variables|/Script/Engine.CharacterMovementComponent|GetMaxWalkSpeedCrouched _soldiermovement))))
      (Variables|Default|SetIncreasedWalkSpeed (* _maxwalkspeed _returnvalue))
      (Variables|Default|SetIncreasedCrouchSpeed (* _output_get_2 _returnvalue))
      (Variables|Default|SetIncreasedProneSpeed (* _output_get _returnvalue))
      (Variables|/Script/Squad.SQSoldierMovement|SetSprintSpeedMultiplier _soldiermovement 3.0)
      (Variables|/Script/Squad.SQSoldierMovement|SetSprintPenalty _soldiermovement 31.0)
      (Variables|/Script/Squad.SQSoldierMovement|SetStaminaRegenRate _soldiermovement 25.0))
    (:then_5
      (CallFunction|UpdateZombieParams))))

(event Custom|ZombieLoop
  (Variables|Default|SetZombieCharge (Math|Float|Clamp(Float) (- (Variables|Default|GetZombieCharge) 25.0) 0.0 (Variables|Default|GetZombieChargeMax))))

(event Custom|ClientBeginPlay
  (Utilities|FlowControl|Delay 3.0)
  (Default|CallPostclientBeginPlay)
  (Variables|Default|SetbClientHasBegunPlay true))

(event Custom|OnSoldierDied_Event_0
  (params (DeadSoldier :type PS%20Soldier%20Object%20Reference) (Killer :type Pawn%20Object%20Reference) (DamageCauser :type Actor%20Object%20Reference) (bPointDamage :type Boolean))
  (bind _horrorsound (Variables|Default|GetHorrorSound))
  (bind _zombiehud (Variables|Default|GetzombieHud))
  (bind _playerstate (Variables|Default|GetPlayerState))
  (Utilities|IsValid _playerstate
    (:Is%20Valid
      (Variables|Default|SetSavedPS _playerstate))
    (:Is%20Not%20Valid
      _))
  (Utilities|FlowControl|Sequence
    (:then_0
      (Components|DestroyComponent (Variables|Default|GetPostProcess))
      (bind _asbp_player_state_crp (Utilities|Casting|CastToBP_PlayerState_CRP (Variables|Default|GetSavedPS)))
      (Variables|/Community_Resource_Pack/Gameplay/Gamemodes/CRPMain/BP_PlayerState_CRP.BP_PlayerState_CRP_C|SetDeadBody _asbp_player_state_crp self)
      (Utilities|IsValid _horrorsound
        (:Is%20Valid
          (Audio|Components|Audio|FadeOut _horrorsound 5.0 0.0 :!class /Script/Engine.AudioComponent)
          (Components|DestroyComponent _horrorsound)
          (Utilities|IsValid _zombiehud
            (:Is%20Valid
              (Widget|RemovefromParent _zombiehud))))))
    (:then_1
      (bind _asbp_player_state_crp_2 (Utilities|Casting|CastToBP_PlayerState_CRP (Variables|Default|GetSavedPS)))
      (bind _asbp_ps_soldier_z (Utilities|Casting|CastToBP_PS_Soldier_Z Killer)
        (:then
          (if (not (Variables|Default|GetbIsZombie))
            (if (Variables|BP_PS_Soldier_Z_C|GetbIsZombie _asbp_ps_soldier_z)
              (Default|SurvivorKilledbyZombie _asbp_player_state_crp_2 self _asbp_ps_soldier_z)
              (else
                (Default|PlayerKilled _asbp_player_state_crp_2 :!label _label)
                (Variables|/Community_Resource_Pack/Gameplay/Gamemodes/CRPMain/BP_PlayerState_CRP.BP_PlayerState_CRP_C|SetDeadBody _asbp_player_state_crp_2 _asbp_ps_soldier_z)))))
        (:CastFailed
          (goto _label))))))

(event EventBeginPlay
  (|CallParentFunction)
  (Utilities|FlowControl|Sequence
    (:then_0
      (Networking|SwitchHasAuthority
        (:Remote
          (if (Pawn|IsLocallyControlled)
            (CallFunction|ClientBeginPlay)))))
    (:then_1
      (EventDispatchers|AssignOnSoldierDied (delegate Custom|OnSoldierDied_Event_0)))
    (:then_2
      (if (Variables|Default|GetbIsZombie)
        (CallFunction|Zombify false)))
    (:then_3
      (bind _aspsplayer_state (Utilities|Casting|CastToPSPlayerState (Variables|Default|GetPlayerState)))
      (if (Math|Boolean|ANDBoolean (!= (Variables|/Script/Squad.SQTeamState|GetId (Class|SQPlayerState|GetTeamState _aspsplayer_state)) 1) (not (Variables|Default|GetbIsZombie)) (Pawn|IsLocallyControlled))
        (bind _returnvalue (UserInterface|CreateWidget "/Community_Resource_Pack/UI/UMG_SoldierNotification_z.UMG_SoldierNotification_Z_C" (Game|GetPlayerController 0)))
        (UserInterface|Viewport|AddtoViewport _returnvalue 0)))))

(event Game|Damage|EventAnyDamage
  (params (Damage :type Float%20%28single-precision%29) (DamageType :type Damage%20Type%20Object%20Reference) (InstigatedBy :type Controller%20Object%20Reference) (DamageCauser :type Actor%20Object%20Reference))
  (|CallParentFunction Damage DamageType InstigatedBy DamageCauser)
  (if (or (!= InstigatedBy (Pawn|GetController)) (Variables|Default|GetbIsZombie))
    (Variables|Default|SetLastDamageTime (Utilities|Time|GetTimeSeconds))
    (Variables|Default|SetZombieCharge (Math|Float|Clamp(Float) (+ (Variables|Default|GetZombieCharge) (* Damage 2.0)) 0.0 (Variables|Default|GetZombieChargeMax)))))

(event Game|Damage|EventPointDamage
  (params (Damage :type Float%20%28single-precision%29) (DamageType :type Damage%20Type%20Object%20Reference) (HitLocation :type Vector :default "0, 0, 0") (HitNormal :type Vector :default "0, 0, 0") (HitComponent :type Primitive%20Component%20Object%20Reference) (BoneName :type Name :default "None") (ShotFromDirection :type Vector :default "0, 0, 0") (InstigatedBy :type Controller%20Object%20Reference) (DamageCauser :type Actor%20Object%20Reference) (HitInfo :type Hit%20Result%20Structure%20%28by%20ref%29))
  (|CallParentFunction Damage DamageType HitLocation HitNormal HitComponent BoneName ShotFromDirection InstigatedBy DamageCauser HitInfo))

(event EventBPWound
  (params (KillingDamage :type Float%20%28single-precision%29) (DamageEvent :type Damage%20Event%20Structure%20%28by%20ref%29) (Killer :type Controller%20Object%20Reference) (DamageCauser :type Actor%20Object%20Reference))
  (|CallParentFunction KillingDamage DamageEvent Killer DamageCauser)
  (Networking|SwitchHasAuthority
    (:Authority
      (Variables|Default|SetSavedPS (Variables|Default|GetPlayerState))
      (if (not (Variables|Default|GetbIsDying))
        (if (Variables|Default|GetbIsZombie)
          (Class|SQSoldier|Die KillingDamage DamageEvent Killer DamageCauser :!label _label)
          (else
            (bind _asbp_ps_soldier_z (Utilities|Casting|CastToBP_PS_Soldier_Z (Pawn|GetControlledPawn Killer)))
            (if (Variables|BP_PS_Soldier_Z_C|GetbIsZombie _asbp_ps_soldier_z)
              (goto _label))))))))

(event EventTick
  (params (DeltaSeconds :type Float%20%28single-precision%29))
  (|CallParentFunction DeltaSeconds))

(fn ConstructionScript
  (|CallParentFunction)
  (Variables|Default|SetDefaultSprintSpeedMultiplier (Variables|/Script/Squad.SQSoldierMovement|GetSprintSpeedMultiplier (Variables|Default|GetSoldierMovement))))

(fn GiveZombieRole
  (bind _returnvalue (Game|ConstructObjectfromClass "/Script/PostScriptum.PSRoleSettings" self))
  (Utilities|Array|SetArrayElem (Variables|/Script/Squad.SQRoleSettings|GetTestInventory _returnvalue) 0 (Utilities|Struct|MakeSQInventoryWeaponGroupData (Utilities|Array|MakeArray (Utilities|Struct|MakeSQInventoryData "/Community_Resource_Pack/Weapons/Z/BP_ZombieMeleeWeapon_Z.BP_ZombieMeleeWeapon_Z_C" false "Primary"))) true)
  (bind _aspsplayer_state (Utilities|Casting|CastToPSPlayerState (Variables|/Script/Engine.Pawn|GetPlayerState self)))
  (Class|SQPlayerState|SetCurrentRole _aspsplayer_state _returnvalue)
  (Class|SQSoldier|SpawnInventory "SwappingRoles"))

(fn OnRepBIsZombie)

(fn GetMaxHealthBP
  (if (Variables|Default|GetbIsZombie)
    (return (Variables|Default|GetMaxZombieHealth))
    (else
      (bind _returnvalue (|CallParentFunction))
      (return _returnvalue))))

(fn OnRepZombieCharge
  (CallFunction|UpdateZombieParams))

(fn UpdateZombieParams
  (bind _soldiermovement (Variables|Default|GetSoldierMovement))
  (if (Variables|Default|GetbIsZombie)
    (Variables|/Script/Engine.CharacterMovementComponent|SetMaxWalkSpeed _soldiermovement (Math|Float|Lerp (Variables|Default|GetIncreasedWalkSpeed) (Variables|Default|GetDefaultWalkSpeed) (/ (Variables|Default|GetZombieCharge) (Variables|Default|GetZombieChargeMax))))
    (Variables|/Script/Engine.CharacterMovementComponent|SetMaxWalkSpeedCrouched _soldiermovement (Math|Float|Lerp (Variables|Default|GetIncreasedCrouchSpeed) (Variables|Default|GetdefaultCrouchSpeed) (/ (Variables|Default|GetZombieCharge) (Variables|Default|GetZombieChargeMax))))
    (Variables|/Script/Squad.SQSoldierMovement|SetMaxWalkSpeedProne _soldiermovement (Math|Float|Lerp (Variables|Default|GetIncreasedProneSpeed) (Variables|Default|GetDefaultProneSpeed) (/ (Variables|Default|GetZombieCharge) (Variables|Default|GetZombieChargeMax))))
    (Networking|SwitchHasAuthority
      (:Authority
        (if (>= (- (Utilities|Time|GetTimeSeconds) (Variables|Default|GetLastDamageTime)) (Variables|Default|GetZombieBleedStopTime))
          (if (Variables|Default|GetbIsBleeding)
            (Class|SQSoldier|StopBleeding)
            (else
              (Class|SQSoldier|Heal (Variables|Default|GetZombieHealthRegenPerSec)))))))))

(fn CanInteractBP
  (if (Variables|Default|GetbIsZombie)
    (return false)
    (else
      (bind _returnvalue (|CallParentFunction))
      (return _returnvalue))))

(fn GorifyMesh
  (bind _mesh (Variables|Character|GetMesh))
  (bind _mesh1p (Variables|Default|GetMesh1P))
  (bind _zombieheadmats (Variables|Default|GetZombieHeadMats))
  (bind _uppermesh1p (Variables|Default|GetUpperMesh1P))
  (bind _returnvalue (Class|SQBlueprintLibrary|GetDefaultObjectfor (Variables|Default|GetGoreMatTable)))
  (bind _asgore_mat_map_table (Utilities|Casting|CastToGoreMatMapTable _returnvalue))
  (for _index (range 0 (- (Rendering|Material|GetNumMaterials _mesh) 1))
    (if (.ReturnValue (Utilities|Map|Find _zombieheadmats (Rendering|Material|GetMaterial _mesh _index)))
      (Rendering|Material|SetMaterial _mesh _index (.Value (Utilities|Map|Find _zombieheadmats (Rendering|Material|GetMaterial _mesh _index))))
      (elif (.ReturnValue (Utilities|Map|Find (Variables|/Script/PostScriptum.GoreMatMapTable|GetGoreSlotMaterials _asgore_mat_map_table) (Rendering|Material|GetMaterial _mesh _index)))
        (Rendering|Material|SetMaterial _mesh _index (.Value (Utilities|Map|Find (Variables|/Script/PostScriptum.GoreMatMapTable|GetGoreSlotMaterials _asgore_mat_map_table) (Rendering|Material|GetMaterial _mesh _index)))))))
  (for _index_2 (range 0 (- (Rendering|Material|GetNumMaterials _mesh1p) 1))
    (if (.ReturnValue (Utilities|Map|Find _zombieheadmats (Rendering|Material|GetMaterial _mesh1p _index_2)))
      (Rendering|Material|SetMaterial _mesh1p _index_2 (.Value (Utilities|Map|Find _zombieheadmats (Rendering|Material|GetMaterial _mesh1p _index_2))))
      (elif (.ReturnValue (Utilities|Map|Find (Variables|/Script/PostScriptum.GoreMatMapTable|GetGoreSlotMaterials _asgore_mat_map_table) (Rendering|Material|GetMaterial _mesh1p _index_2)))
        (Rendering|Material|SetMaterial _mesh1p _index_2 (.Value (Utilities|Map|Find (Variables|/Script/PostScriptum.GoreMatMapTable|GetGoreSlotMaterials _asgore_mat_map_table) (Rendering|Material|GetMaterial _mesh1p _index_2)))))))
  (for _index_3 (range 0 (- (Rendering|Material|GetNumMaterials _uppermesh1p) 1))
    (if (.ReturnValue (Utilities|Map|Find _zombieheadmats (Rendering|Material|GetMaterial _uppermesh1p _index_3)))
      (Rendering|Material|SetMaterial _uppermesh1p _index_3 (.Value (Utilities|Map|Find _zombieheadmats (Rendering|Material|GetMaterial _uppermesh1p _index_3))))
      (elif (.ReturnValue (Utilities|Map|Find (Variables|/Script/PostScriptum.GoreMatMapTable|GetGoreSlotMaterials _asgore_mat_map_table) (Rendering|Material|GetMaterial _uppermesh1p _index_3)))
        (Rendering|Material|SetMaterial _uppermesh1p _index_3 (.Value (Utilities|Map|Find (Variables|/Script/PostScriptum.GoreMatMapTable|GetGoreSlotMaterials _asgore_mat_map_table) (Rendering|Material|GetMaterial _uppermesh1p _index_3)))))))
  (return _mesh))

(fn OnRepAttachedtoVehicle
  (bind _attachedtovehicle (Variables|Default|GetAttachedToVehicle))
  (bind _capsulecomponent (Variables|Default|GetCapsuleComponent))
  (bind _soldiermovement (Variables|Default|GetSoldierMovement))
  (Utilities|IsValid _attachedtovehicle
    (:Is%20Valid
      (Variables|Default|SetLastAttachedVehicle _attachedtovehicle)
      (Pawn|Components|CharacterMovement|DisableMovement (Variables|Default|GetSoldierMovement))
      (Actor|Tick|AddTickPrerequisiteActor _attachedtovehicle)
      (Collision|SetCollisionEnabled _capsulecomponent "NoCollision")
      (Collision|IgnoreActorwhenMoving _capsulecomponent _attachedtovehicle true)
      (Variables|/Script/Engine.CharacterMovementComponent|SetbIgnoreClientMovementErrorChecksAndCorrection _soldiermovement true)
      (if (Pawn|IsLocallyControlled)
        _))
    (:Is%20Not%20Valid
      (Utilities|IsValid (Variables|Default|GetLastAttachedVehicle)
        (:Is%20Valid
          (Pawn|Components|CharacterMovement|SetMovementMode (Variables|Default|GetSoldierMovement) "MOVE_Walking" 0)
          (Class|Actor|RemoveTickPrerequisiteActor (Variables|Default|GetLastAttachedVehicle))
          (Collision|SetCollisionEnabled _capsulecomponent "QueryOnly")
          (Collision|IgnoreActorwhenMoving _capsulecomponent (Variables|Default|GetLastAttachedVehicle) false)
          (Variables|/Script/Engine.CharacterMovementComponent|SetbIgnoreClientMovementErrorChecksAndCorrection _soldiermovement false)
          (Transformation|SetActorRelativeRotation (Math|Rotator|MakeRotator 0.0 0.0 (.Yaw (Math|Rotator|BreakRotator (Transformation|GetActorRotation)))))
          (bind _asbp_player_controller (Utilities|Casting|CastToBP_PlayerController (Pawn|GetController)))
          (Pawn|SetControlRotation _asbp_player_controller (Math|Rotator|MakeRotator 0.0 0.0 0.0))
          (if (Pawn|IsLocallyControlled)
            _))))))

(fn UpgradeZombieMesh
  (for _index (range 0 (- (Rendering|Material|GetNumMaterials (Variables|Character|GetMesh)) 1))
    (if (.ReturnValue (Utilities|Map|Find (Variables|Default|GetZombieHeadMatsUpgraded) (Rendering|Material|GetMaterial (Variables|Character|GetMesh) _index)))
      (Rendering|Material|SetMaterial (Variables|Character|GetMesh) _index (.Value (Utilities|Map|Find (Variables|Default|GetZombieHeadMatsUpgraded) (Rendering|Material|GetMaterial (Variables|Character|GetMesh) _index)))))))
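; Game state Blueprint for the CRP OffensiveChild gamemode, configuring feature switches and the commander check through small functions.
; It reports offensive features as off and vanilla armored features as on, despite the Offensive name.
; The CRP commander check passes for any player who is a squad leader.
; It adds no event logic of its own, as BeginPlay and Tick are disabled placeholders.
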(event EventBeginPlay
  (|CallParentFunction) ; This node is disabled and will not be called.\nDrag off pins to build functionality.
)

(event EventTick
  (params (DeltaSeconds :type Float%20%28single-precision%29))
  (|CallParentFunction DeltaSeconds) ; This node is disabled and will not be called.\nDrag off pins to build functionality.
)

(fn ConstructionScript
  (|CallParentFunction))

(fn UseOffensiveFeatures
  (return 0))

(fn UseVanillaArmoredFeatures
  (return 1))

(fn CheckPlayerIsCommanderCRP
  (params (Player :type BP%20Player%20Controller%20Object%20Reference))
  (return (Class|SQPlayerController|IsSquadLeader Player)))
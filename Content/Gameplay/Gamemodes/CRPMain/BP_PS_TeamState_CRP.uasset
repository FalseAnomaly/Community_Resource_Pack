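; Team state for the CRP game mode that overrides squad limits when the game state enables its "Z features", otherwise using parent logic.
; In that mode, the listed squad types share one pool, each limited to the allowance minus the other types' counts.
; The allowance is recalculated from player count, survivor ratio and squad size, only growing within a clamped range.
; Code to create blank UK/US/FR survivor squads is present but disconnected.
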(event EventBeginPlay
  (|CallParentFunction) ; This node is disabled and will not be called.\nDrag off pins to build functionality.
)

(event EventTick
  (params (DeltaSeconds :type Float%20%28single-precision%29)))

(fn ConstructionScript
  (|CallParentFunction))

(fn GetCurrentSquadLimit
  (params (Type :type EPSSquadType%20Enum :default "Commander"))
  (bind _returnvalue (Game|GetGameState))
  (if (Utilities|DoesObjectImplementInterface _returnvalue "/Community_Resource_Pack/Gameplay/Gamemodes/CRPMain/BPI_GameState_CRP.BPI_GameState_CRP_C")
    (bind _return_value (Class|BPIGameStateCRP|UseZFeatures(Message) _returnvalue))
    (if _return_value
      (for _array_element (Utilities|Array|MakeArray "Commander" "Infantry" "Logistics" "Armor" "Armored_Recon" "Armored_Tank" "Armored_Commander")
        (if (!= Type _array_element)
          (LocalVariables|SetSum (+ (LocalVariables|GetSum) (Class|PSTeamState|GetCurrentSquadCount _array_element)))))
      (return (- (Variables|Default|GetCurrentAllowedInfantrySquadCountZ) (LocalVariables|GetSum)))
      (else
        (return (|CallParentFunction Type))))))

(fn ReCalculateSquadLimits
  (LocalVariables|SetRequiredSurvivors (* (Utilities|Array|Length (Variables|/Script/Engine.GameStateBase|GetPlayerArray (Game|GetGameState))) (Variables|Default|GetSurvivorSquadRatioZ)))
  (bind _output_get (Variables|Default|SetCurrentAllowedInfantrySquadCountZ (Math|Integer|Clamp(Integer) (Math|Integer|Max(Integer) (Math|Float|Ceil (/ (LocalVariables|GetRequiredSurvivors) (Math|Conversions|ToFloat(Integer) (Variables|Default|GetSquadSizeZ)))) (Variables|Default|GetCurrentAllowedInfantrySquadCountZ)) 1 12)))
  (bind _output_get_2 (LocalVariables|SetExisitngSquadGroupCount (/ (Utilities|Array|Length (Variables|Default|GetSquadStates)) 3))))

(fn GetCurrentSquadCountCRP
  (params (Type :type EPSSquadType%20Enum :default "Commander"))
  (return (Class|PSTeamState|GetCurrentSquadCount Type)))
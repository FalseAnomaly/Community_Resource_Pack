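; Game state for the CRP main gamemode, defining team sections, squad sizes, rally permission and commander checks.
; Mode feature queries return off, including UseZFeatures, which gates creation of the Z objective status widget at BeginPlay.
; The player's radial menu class comes from their team info, and replicated crew counts trigger an update call.
; Events handle toasts with an alert sound, delayed important-event sounds and actor destruction.
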(event Custom|ToastAll
  (params (ToastText :type Text))
  (Networking|CanExecuteCosmeticEvents
    (:True
      (bind _assqplayer_controller (Utilities|Casting|CastToSQPlayerController (Game|GetPlayerController 0)))
      (Class|SQPlayerController|ShowToast _assqplayer_controller ToastText 5.0 false)
      (Audio|SpawnSound2D self (Variables|Default|GetImportantEventSound) 1.0 1.0 0.0 0))))

(event Custom|SignalImportantEvent
  (params (Delay :type Float%20%28single-precision%29))
  (Utilities|FlowControl|Delay Delay)
  (Audio|SpawnSound2D self (Variables|Default|GetImportantEventSound) 1.0 1.0 0.0 0))

(event Custom|RepDestroy
  (params (Input%20Actor :type Actor%20Object%20Reference))
  (Actor|DestroyActor Input%20Actor))

(event EventBeginPlay
  (|CallParentFunction)
  (bind _return_value (CallFunction|UseZFeatures))
  (if _return_value
    (Networking|CanExecuteCosmeticEvents
      (:True
        (bind _returnvalue (UserInterface|CreateWidget "/Community_Resource_Pack/UI/UMG_ObjectiveStatusDisplay_Z.UMG_ObjectiveStatusDisplay_Z_C" (Game|GetPlayerController 0)))
        (bind _output_get (Variables|Default|SetObjectiveStateWidgetZ _returnvalue))
        (UserInterface|Viewport|AddtoViewport _output_get 0)))))

(event EventTick
  (params (DeltaSeconds :type Float%20%28single-precision%29)))

(fn ConstructionScript
  (|CallParentFunction))

(fn OnRepTeamCrewCounts
  (Default|CallOnCrewCountUpdateCRP))

(fn AllowRallies
  (return true))

(fn AllowTeamSection
  (params (TeamID :type Integer) (Squad%20Type :type EPSSquadType%20Enum :default "Commander"))
  (return true))

(fn CheckPlayerIsCommanderCRP
  (params (Player :type BP%20Player%20Controller%20Object%20Reference))
  (bind _squadstate (Variables|/Script/Squad.SQPlayerController|GetSquadState Player))
  (Utilities|IsValid _squadstate
    (:Is%20Valid
      (bind _asbp_ps_squad_state (Utilities|Casting|CastToBP_PS_SquadState _squadstate)
        (:then
          (if (Utilities|Enum|Equal(Enum) (Variables|/Script/PostScriptum.PSSquadState|GetSquadType _asbp_ps_squad_state) "Commander")
            (if (Class|SQPlayerController|IsSquadLeader Player)
              (return true)
              (else
                _))))
        (:CastFailed
          _)))
    (:Is%20Not%20Valid
      _))
  (return false))

(fn GetPlayerRadialMenuClass
  (params (Player :type Player%20Controller%20Object%20Reference))
  (bind _asbp_ps_player_controller (Utilities|Casting|CastToBP_PS_PlayerController Player)
    (:then
      (if (Utilities|IsValid (Variables|/Script/Squad.SQPlayerController|GetTeamState _asbp_ps_player_controller))
        (bind _asbp_ps_team_info (Utilities|Casting|CastToBP_PS_TeamInfo (Variables|/Script/Squad.SQTeamState|GetInfo (Variables|/Script/Squad.SQPlayerController|GetTeamState _asbp_ps_player_controller)))
          (:then
            (bind _menuclass (Default|GetPSCommandMenuClass _asbp_ps_team_info _asbp_ps_player_controller))
            (return _menuclass))
          (:CastFailed
            _))))
    (:CastFailed
      _))
  (return 0))

(fn GetSectionsDisplayImage
  (params (TeamID :type Integer))
  (return (Utilities|Array|MakeArray "/Game/PostScriptum/UI/Vehicles/VehiclesMapIcons/Inverted/map_commander.map_commander" "/Game/PostScriptum/UI/Vehicles/VehiclesMapIcons/W_Faction_Infantry.W_Faction_Infantry" "/Game/PostScriptum/UI/Vehicles/VehiclesMapIcons/W_Faction_Logistic.W_Faction_Logistic" "/Game/PostScriptum/UI/Vehicles/VehiclesMapIcons/W_Faction_Tank.W_Faction_Tank" "/Game/PostScriptum/UI/Vehicles/VehiclesMapIcons/W_Faction_Infantry.W_Faction_Infantry" "/Game/PostScriptum/UI/Vehicles/VehiclesMapIcons/W_Faction_Infantry.W_Faction_Infantry")))

(fn GetSectionsDisplayName
  (params (TeamID :type Integer))
  (return (Utilities|Array|MakeArray "Commander" "Infantry" "Logistics" "Armored" "Custom 1" "Custom 2")))

(fn GetTeamSquadSize
  (params (TeamID :type Integer) (Squad%20Type :type EPSSquadType%20Enum :default "Commander"))
  (return (Utilities|Select :Index Squad%20Type :Commander 4 :Infantry 9 :Logistics 4 :Armor 4 :Armored_Recon -1 :Armored_Tank -1 :Armored_Commander -1)))

(fn GetZHumanTeam
  (return 2))

(fn SectionListShowDeadPlayers
  (return false))

(fn UseCRPArmoredFeatures
  (return 0))

(fn UseInvasionFeatures
  (return 0))

(fn UseOffensiveFeatures
  (return 0))

(fn UseRAASFeatures
  (return 0))

(fn UseSupremacyFeatures
  (return 0))

(fn UseVanillaArmoredFeatures
  (return 0))

(fn UseZFeatures
  (return false))
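; CRP gamemode player controller that overrides squad-leaving and support-call rules through queries to the game state's BPI_GameState_CRP interface.
; With Z features on, members of the Z human team cannot leave their squad.
; Support calls use either the parent check or CRP commander status plus IsInRadioRange, whose parent call is unreachable, so it never returns true.
; CRP squad-creation and role-deploy functions simply forward to the base calls.
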(event Custom|Init
  (if (not (Variables|Default|GetbInitialized))
    (|CallParentFunction)
    (Variables|Default|SetbInitialized true)))

(event EventBeginPlay
  (|CallParentFunction)
  (Variables|Default|SetbInitialized true))

(event EventTick
  (params (DeltaSeconds :type Float%20%28single-precision%29)))

(event EventCreateIntermediateLoadingScreenifNecessary)

(fn ConstructionScript
  (|CallParentFunction))

(fn CanLeaveCurrentSquad
  (bind _returnvalue (Game|GetGameState))
  (if (Utilities|DoesObjectImplementInterface _returnvalue "/Community_Resource_Pack/Gameplay/Gamemodes/CRPMain/BPI_GameState_CRP.BPI_GameState_CRP_C")
    (bind _return_value (Class|BPIGameStateCRP|UseZFeatures(Message) _returnvalue))
    (if _return_value
      (bind _human_teamid (Class|BPIGameStateCRP|GetZHumanTeam(Message) _returnvalue))
      (if (== _human_teamid (Class|SQTeamInterface|GetTeamId))
        (return false)
        (else
          _))))
  (return (|CallParentFunction)))

(fn IsinRadioRange
  (bind _returnvalue (Game|GetGameState))
  (if (Utilities|DoesObjectImplementInterface _returnvalue "/Community_Resource_Pack/Gameplay/Gamemodes/CRPMain/BPI_GameState_CRP.BPI_GameState_CRP_C")
    (bind _return_value (Class|BPIGameStateCRP|UseZFeatures(Message) _returnvalue))
    (if _return_value
      (return false))))

(fn CanCallSupport
  (bind _returnvalue (Game|GetGameState))
  (bind _self self)
  (if (Utilities|DoesObjectImplementInterface _returnvalue "/Community_Resource_Pack/Gameplay/Gamemodes/CRPMain/BPI_GameState_CRP.BPI_GameState_CRP_C")
    (bind _return_value (Class|BPIGameStateCRP|UseVanillaCommanderCheck(Message) _returnvalue))
    (if _return_value
      _
      (else
        (bind _is_commander (Class|BPIGameStateCRP|CheckPlayerIsCommanderCRP(Message) _returnvalue _self))
        (return (and (CallFunction|IsinRadioRange _self) _is_commander)))))
  (bind _return (|CallParentFunction))
  (return _return))

(fn CreateSquadCRP
  (params (Type :type EPSSquadType%20Enum :default "Commander") (Size :type Integer) (Name :type String))
  (Class|PSPlayerController|CreatePSSquad Type Size Name))

(fn ServerRequestDeployRoleCRP
  (params (New%20Role :type SQ%20Role%20Settings%20Object%20Reference))
  (if (Class|SQPlayerController|IsSquadLeader self)
    _
    (else
      _))
  (Class|SQPlayerController|ServerRequestDeployRole New%20Role))
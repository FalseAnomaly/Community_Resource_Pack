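; BP_PSSquadState_CRP is the squad state Blueprint for the CRP main game mode, customizing how the squad reports its player count.
; It overrides GetNumPlayerCount, querying the game state through BPI_GameState_CRP for whether Z features are in use.
; When they are, it adds the number of KilledPlayerInfos entries to the parent's count; otherwise it returns the parent's count unchanged.
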(event EventBeginPlay)

(event EventTick
  (params (DeltaSeconds :type Float%20%28single-precision%29)))

(fn ConstructionScript)

(fn GetNumPlayerCount
  (bind _returnvalue (Game|GetGameState))
  (bind _count (|CallParentFunction))
  (if (Utilities|DoesObjectImplementInterface _returnvalue "/Community_Resource_Pack/Gameplay/Gamemodes/CRPMain/BPI_GameState_CRP.BPI_GameState_CRP_C")
    (bind _return_value (Class|BPIGameStateCRP|UseZFeatures(Message) _returnvalue))
    (if _return_value
      (return (+ (Utilities|Array|Length (Variables|Default|GetKilledPlayerInfos)) _count))
      (else
        _)))
  (return _count))
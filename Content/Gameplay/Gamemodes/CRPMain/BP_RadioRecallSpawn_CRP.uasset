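; CRP variant of a radio recall spawn actor that blocks itself when the game mode disallows rally points.
; On BeginPlay it queries the game state through BPI_GameState_CRP, running parent startup if rallies are allowed or the interface is absent.
; Otherwise it destroys itself, with the server first sending the squad leader a "Rally points disabled!" warning.
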(event EventTick
  (params (DeltaSeconds :type Float%20%28single-precision%29))
  (|CallParentFunction DeltaSeconds) ; This node is disabled and will not be called.\nDrag off pins to build functionality.
)

(event EventBeginPlay
  (bind _returnvalue (Game|GetGameState))
  (if (Utilities|DoesObjectImplementInterface _returnvalue "/Community_Resource_Pack/Gameplay/Gamemodes/CRPMain/BPI_GameState_CRP.BPI_GameState_CRP_C")
    (bind _return_value (Class|BPIGameStateCRP|AllowRallies(Message) _returnvalue))
    (if _return_value
      (|CallParentFunction :!label _label)
      (else
        (Networking|SwitchHasAuthority
          (:Authority
            (bind _assqplayer_controller (Utilities|Casting|CastToSQPlayerController (Pawn|GetController (Variables|/Script/Squad.SQPlayerState|GetCurrentPawn (Variables|/Script/Squad.SQSquadState|GetLeaderState (Variables|Default|GetSquadState)))))
              (:then
                (Class|SQPlayerController|ClientChat _assqplayer_controller 0 "Rally points disabled!" "GameNotification" "Warning"))
              (:CastFailed
                _)))
          (:Remote
            _))
        (Actor|DestroyActor)))
    (else
      (goto _label))))

(fn ConstructionScript
  (|CallParentFunction))
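; Player state for the CRP zombie game mode that converts killed survivors to the zombie team and notifies their squad of the death.
; A zombie kill also records the body and class, then starts rising-soul and delayed timers on the server.
; RespawnAsZombie restarts the player at a short-lived spawn point created on the corpse, then removes the body.
; The zombie upgrade function exists, but its call is unconnected.
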(event Custom|RespawnAsZombie
  (bind _deadbody (Variables|Default|GetDeadBody))
  (Utilities|FlowControl|Sequence
    (:then_0
      (Networking|SwitchHasAuthority
        (:Authority
          (Variables|Default|SetbShouldSpawn true)
          (bind _assqplayer_controller (Utilities|Casting|CastToSQPlayerController (Components|GetOwner)))
          (bind _returnvalue (Game|SpawnActorfromClass "/Community_Resource_Pack/Gameplay/Gamemodes/CRPMain/BP_SQGameSpawn_Temp_CRP.BP_SQGameSpawn_Temp_CRP_C" (Math|Transform|MakeTransform (Transformation|GetActorLocation (Variables|Default|GetDeadBody))) "AdjustIfPossibleButAlwaysSpawn" 0 0))
          (bind _output_get (Variables|Default|SetSurvivorZombieRevivePoint _returnvalue))
          (Actor|SetLifeSpan _output_get 0.5)
          (Class|SQGameSpawn|SetTeam _output_get "Team_One")
          (Class|SQPlayerController|ServerRequestRestartPlayer _assqplayer_controller _output_get))))
    (:then_1
      (Utilities|IsValid _deadbody
        (:Is%20Valid
          (Actor|DestroyActor _deadbody))))))

(event Custom|PlayerKilled
  (bind _squadstate (Variables|Default|GetSquadState))
  (Utilities|FlowControl|Sequence
    (:then_0
      (Utilities|IsValid _squadstate
        (:Is%20Valid
          (bind _asbp_ps_squad_crp (Utilities|Casting|CastToBP_PS_Squad_CRP (Variables|/Script/Squad.SQSquadState|GetAuthoritySquad _squadstate)))
          (Default|SquadMemberKilled _asbp_ps_squad_crp self))))
    (:then_1
      (CallFunction|SwitchtoZombie))))

(event Custom|SpawnSoul)

(event EventTick
  (params (DeltaSeconds :type Float%20%28single-precision%29)))

(fn ConstructionScript)

(fn SurvivorKilledbyZombie
  (params (KilledSoldier :type BP%20PS%20Soldier%20Z%20Object%20Reference) (KillerZombie :type Pawn%20Object%20Reference))
  (bind _squadstate (Variables|Default|GetSquadState))
  (Utilities|FlowControl|Sequence
    (:then_0
      (Variables|Default|SetDeadBody KilledSoldier)
      (Networking|SwitchHasAuthority
        (:Authority
          (Variables|Default|SetSurvivorCharacterClass (Utilities|GetClass KilledSoldier))
          (Variables|Default|SetbSurvivorKilledByZombie true)
          (Utilities|IsValid _squadstate
            (:Is%20Valid
              (bind _asbp_ps_squad_crp (Utilities|Casting|CastToBP_PS_Squad_CRP (Variables|/Script/Squad.SQSquadState|GetAuthoritySquad _squadstate))
                (:then
                  (Default|SquadMemberKilled _asbp_ps_squad_crp self))
                (:CastFailed
                  _)))
            (:Is%20Not%20Valid
              _))
          (CallFunction|SwitchtoZombie)
          (Utilities|Time|SetTimerbyFunctionName KilledSoldier "SpawnRisingSoul" 2.0)
          (Utilities|Time|SetTimerbyEvent (EventDispatchers|CreateEvent :!event Custom|RespawnAsZombie) 1e+01)
          (Variables|Default|SetbShouldSpawn false))))))

(fn OnPlayerRevivedasZombie
  (bind _survivorzombierevivepoint (Variables|Default|GetSurvivorZombieRevivePoint))
  (bind _deadbody (Variables|Default|GetDeadBody))
  (Utilities|FlowControl|Sequence
    (:then_0
      (Utilities|IsValid _survivorzombierevivepoint
        (:Is%20Valid
          (Actor|DestroyActor _survivorzombierevivepoint))))
    (:then_1
      (Utilities|IsValid _deadbody
        (:Is%20Valid
          (Actor|DestroyActor _deadbody))))
    (:then_2
      (Variables|Default|SetbSurvivorKilledByZombie false))))

(fn SwitchtoZombie
  (bind _asbp_ps_game_mode_z (Utilities|Casting|CastToBP_PS_GameMode_Z (Game|GetGameMode)))
  (bind _asbp_player_controller (Utilities|Casting|CastToBP_PlayerController (Components|GetOwner)))
  (Class|SQGameMode|TrytoChangePlayersTeam _asbp_ps_game_mode_z _asbp_player_controller (Variables|/Community_Resource_Pack/Gameplay/Gamemodes/Z/BP_PS_GameMode_Z.BP_PS_GameMode_Z_C|GetZombieTeamId _asbp_ps_game_mode_z) true))

(fn UpgradeZombie
  (params (Target%20Zombie :type Pawn%20Object%20Reference))
  (bind _assqplayer_controller (Utilities|Casting|CastToSQPlayerController (Game|GetPlayerController 0)))
  (Class|SQPlayerController|ShowToast _assqplayer_controller (Variables|Default|GetZombieUpgradeText) 5.0 false)
  (Utilities|Time|SetTimerbyFunctionName Target%20Zombie "UpgradeZombieMesh" 5.0))
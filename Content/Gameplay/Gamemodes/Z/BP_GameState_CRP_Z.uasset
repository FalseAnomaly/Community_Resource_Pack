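; Game state for the Z game mode, overriding team, section and menu rules and showing a mode-specific victory display.
; Only team 2 gets sections, with fixed size, faction names and emblems; rallies are disabled and dead players stay listed.
; Team 2 leaders receive the non-build squad-leader radial menu.
; A cosmetic stats event spawns the Z victory display at an existing display's transform, or at the origin without stats.
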(event EventBeginPlay
  (|CallParentFunction) ; This node is disabled and will not be called.\nDrag off pins to build functionality.
)

(event EventTick
  (params (DeltaSeconds :type Float%20%28single-precision%29))
  (|CallParentFunction DeltaSeconds) ; This node is disabled and will not be called.\nDrag off pins to build functionality.
)

(event EventSendStatsMulticast
  (params (bVisible :type Boolean) (WinnerTeam :type Byte :default 0) (Team1Stats :type Processed%20Stats%20Container%20Structure) (Team2Stats :type Processed%20Stats%20Container%20Structure))
  (Networking|CanExecuteCosmeticEvents
    (:True
      (if bVisible
        (bind _outactors (Actor|GetAllActorsOfClass "/Game/PostScriptum/Blueprints/BP_VictoryDisplay.BP_VictoryDisplay_C"))
        (if (> (Utilities|Array|Length _outactors) 0)
          (bind _returnvalue (Game|SpawnActorfromClass "/Community_Resource_Pack/Blueprints/Z/BP_VictoryDisplay_Z.BP_VictoryDisplay_Z_C" (Transformation|GetActorTransform (Utilities|Array|Get(acopy) _outactors)) "AlwaysSpawn" 0 0 0))
          (bind _output_get (Variables|Default|SetVictoryDisplay _returnvalue))
          (Default|Init _output_get WinnerTeam Team1Stats Team2Stats)
          (else
            (bind _returnvalue_2 (Game|SpawnActorfromClass "/Community_Resource_Pack/Blueprints/Z/BP_VictoryDisplay_Z.BP_VictoryDisplay_Z_C" (Math|Transform|MakeTransform "0, 0, 0") "AlwaysSpawn" 0 0 0))
            (bind _output_get_2 (Variables|Default|SetVictoryDisplay _returnvalue_2))
            (Default|Init _output_get_2)))
        (else
          (Utilities|IsValid (Variables|Default|GetVictoryDisplay)
            (:Is%20Valid
              (Default|UnInit (Variables|Default|GetVictoryDisplay)))))))))

(fn ConstructionScript
  (|CallParentFunction))

(fn UseZFeatures
  (return true))

(fn SectionListShowDeadPlayers
  (return true))

(fn AllowRallies
  (return false))

(fn AllowTeamSection
  (params (TeamID :type Integer) (Squad%20Type :type EPSSquadType%20Enum :default "Commander"))
  (switch int TeamID
    (:0
      _)
    (:1
      _)
    (:2
      (return true)))
  (return false))

(fn GetSectionsDisplayName
  (params (TeamID :type Integer))
  (switch int TeamID
    (:Default
      _)
    (:0
      _)
    (:1
      _)
    (:2
      (return (Utilities|Array|MakeArray "UK 1st Airborne" "DE Wehrmacht 1944" "FR 21e DI" "DE Wehrmacht 1940" "US 4th Army" "DE 6. Fallschirmjäger"))))
  (return (Utilities|Array|MakeArray "" "" "" "" "" "")))

(fn GetSectionsDisplayImage
  (params (TeamID :type Integer))
  (switch int TeamID
    (:Default
      _)
    (:0
      _)
    (:1
      _)
    (:2
      (return (Utilities|Array|MakeArray "/Game/PostScriptum/UI/Textures/W_Faction_1st_Airbone.W_Faction_1st_Airbone" "/Game/PostScriptum/UI/Textures/W_Faction_German_censored.W_Faction_German_censored" "/Game/PostScriptum/UI/Textures/W_Faction_FR_Army_21e.W_Faction_FR_Army_21e" "/Game/PostScriptum/UI/Textures/W_Faction_German_censored.W_Faction_German_censored" "/Game/PostScriptum/UI/Textures/W_Faction_4th_Infantry.W_Faction_4th_Infantry" "/Game/PostScriptum/UI/Textures/W_Faction_Fallschirmjager.W_Faction_Fallschirmjager"))))
  (return (Utilities|Array|MakeArray 0 0 0 0 0 0)))

(fn GetPlayerRadialMenuClass
  (params (Player :type Player%20Controller%20Object%20Reference))
  (bind _returnvalue (Class|SQTeamInterface|GetTeamId(Message) Player))
  (if (== _returnvalue 2)
    (bind _asbp_ps_player_controller (Utilities|Casting|CastToBP_PS_PlayerController Player))
    (if (Variables|/Script/Squad.SQRoleSettings|GetbIsLeader (Class|SQPlayerController|GetCurrentRole _asbp_ps_player_controller))
      (bind _asbp_ps_team_info (Utilities|Casting|CastToBP_PS_TeamInfo (Variables|/Script/Squad.SQTeamState|GetInfo (Variables|/Script/Squad.SQPlayerController|GetTeamState _asbp_ps_player_controller)))
        (:then
          (return (Variables|/Game/Gameplay/Teams/BP_TeamInfo.BP_TeamInfo_C|GetNonBuildSLCommandMenu _asbp_ps_team_info)))
        (:CastFailed
          _))))
  (return 0))

(fn GetTeamSquadSize
  (params (TeamID :type Integer) (Squad%20Type :type EPSSquadType%20Enum :default "Commander"))
  (if (== TeamID 2)
    (return 5)
    (else
      (return 0))))
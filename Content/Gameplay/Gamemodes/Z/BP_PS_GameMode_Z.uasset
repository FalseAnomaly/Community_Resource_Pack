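; Game mode for zombies versus survivors that activates random objective spawners and sets zombies as the timeout winner.
; Survivor deaths are recorded in GameState, and the match ends when the checked team has no living players.
; Recorded dead and latecomers past a cutoff are kept off survivors, who also need a squad to spawn.
; Pawn class and start overrides revive zombie-killed survivors with their saved character and revive point, and restart zombifies zombie-team players.
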(event Custom|SoldierDied
  (params (DeadSoldier :type PS%20Soldier%20Object%20Reference) (Killer :type Pawn%20Object%20Reference) (DamageCauser :type Actor%20Object%20Reference) (bPointDamage :type Boolean))
  (bind _aspsgame_state (Utilities|Casting|CastToPSGameState (Game|GetGameState)))
  (bind _asbp_ps_team_state (Utilities|Casting|CastToBP_PS_TeamState (Utilities|Array|Get(acopy) (Variables|/Script/Squad.SQGameState|GetIndexedTeamStates _aspsgame_state) (Utilities|Select :Index (Variables|Default|GetZombieTeamId) :Option%200 0 :Option%201 2 :Option%202 1))))
  (if (not (Default|TeamHasLivePlayers _asbp_ps_team_state))
    (CallFunction|ForceEndMatch (Variables|Default|GetZombieTeamId))))

(event Custom|OnSoldierDied_Event_0
  (params (DeadSoldier :type PS%20Soldier%20Object%20Reference) (Killer :type Pawn%20Object%20Reference) (DamageCauser :type Actor%20Object%20Reference) (bPointDamage :type Boolean))
  (Utilities|FlowControl|Sequence
    (:then_0
      (bind _asbp_ps_soldier_z (Utilities|Casting|CastToBP_PS_Soldier_Z DeadSoldier))
      (bind _assqplayer_state (Utilities|Casting|CastToSQPlayerState (select (Utilities|IsValid (Variables|/Script/Engine.Pawn|GetPlayerState _asbp_ps_soldier_z)) (Variables|/Script/Engine.Pawn|GetPlayerState _asbp_ps_soldier_z) (Variables|/PSCommunityResourcePack/Soldiers/Z/BP_PS_Soldier_Z.BP_PS_Soldier_Z_C|GetSavedPS _asbp_ps_soldier_z))))
      (bind _asbp_game_state_crp (Utilities|Casting|CastToBP_GameState_CRP (Game|GetGameState)))
      (Utilities|Array|Add (Variables|/Community_Resource_Pack/Gameplay/Gamemodes/CRPMain/BP_GameState_CRP.BP_GameState_CRP_C|GetDeadPlayers _asbp_game_state_crp) (Class|SQPlayerState|GetUniqueNetID _assqplayer_state)))
    (:then_1
      (bind _aspsgame_state (Utilities|Casting|CastToPSGameState (Game|GetGameState)))
      (bind _asbp_ps_team_state (Utilities|Casting|CastToBP_PS_TeamState (Utilities|Array|Get(acopy) (Variables|/Script/Squad.SQGameState|GetIndexedTeamStates _aspsgame_state) (Utilities|Select :Index (Variables|Default|GetZombieTeamId) :Option%200 0 :Option%201 2 :Option%202 1))))
      (if (not (Default|TeamHasLivePlayers _asbp_ps_team_state))
        (CallFunction|ForceEndMatch (Variables|Default|GetZombieTeamId))))))

(event EventBeginPlay
  (|CallParentFunction)
  (Utilities|FlowControl|Sequence
    (:then_0
      (bind _outactors (Actor|GetAllActorsOfClass "/Community_Resource_Pack/Blueprints/Z/BP_ObjectiveSpawner_Z.BP_ObjectiveSpawner_Z_C"))
      (bind _output_get (Variables|Default|SetAllObjs _outactors))
      (Variables|Default|SetTotalObjs (Utilities|Array|Length _output_get))
      (for _index (range 0 (- (Variables|Default|GetTotalObjs) 1))
        (if (< (Variables|Default|GetActivatedObjCount) (Variables|Default|GetMaxObjectives))
          (Variables|Default|SetChosen (Utilities|Array|Get(acopy) (Variables|Default|GetAllObjs) (Math|Random|RandomInteger (Utilities|Array|LastIndex (Variables|Default|GetAllObjs)))))
          (Default|Activate (Variables|Default|GetChosen))
          (Utilities|Array|RemoveItem (Variables|Default|GetAllObjs) (Variables|Default|GetChosen))
          (Math|Integer|IncrementInt (Variables|Default|GetActivatedObjCount))))
      (Development|PrintString (Utilities|String|ToString(Integer) (Variables|Default|GetActivatedObjCount))))
    (:then_1
      ;[1 1 1] For cases of timeout
      (Variables|Default|SetForcedEndMatchWinTeam (Variables|Default|GetZombieTeamId)))))

(event EventOnSwapPlayerControllers
  (params (OldPC :type Player%20Controller%20Object%20Reference) (NewPC :type Player%20Controller%20Object%20Reference))
  (|CallParentFunction OldPC NewPC))

(event EventOnRestartPlayer
  (params (NewPlayer :type Controller%20Object%20Reference))
  (|CallParentFunction NewPlayer)
  (bind _returnvalue (Class|SQTeamInterface|GetTeamId(Message) NewPlayer))
  (bind _asbp_ps_soldier_z (Utilities|Casting|CastToBP_PS_Soldier_Z (Pawn|GetControlledPawn NewPlayer)))
  (if (== _returnvalue (Variables|Default|GetZombieTeamId))
    (bind _asbp_player_state_crp (Utilities|Casting|CastToBP_PlayerState_CRP (Variables|/Script/Engine.Pawn|GetPlayerState _asbp_ps_soldier_z)))
    (Default|OnPlayerRevivedasZombie _asbp_player_state_crp)
    (Default|GiveZombieRole _asbp_ps_soldier_z)
    (Default|Zombify _asbp_ps_soldier_z false)
    (else
      (EventDispatchers|AssignOnSoldierDied _asbp_ps_soldier_z (delegate Custom|OnSoldierDied_Event_0)))))

(event EventHandleStartingNewPlayer
  (params (NewPlayer :type Player%20Controller%20Object%20Reference))
  (|CallParentFunction NewPlayer)
  (bind _asbp_ps_player_controller_crp (Utilities|Casting|CastToBP_PS_PlayerController_CRP NewPlayer))
  (Default|Init _asbp_ps_player_controller_crp)
  (bind _aspsgame_state (Utilities|Casting|CastToPSGameState (Game|GetGameState)))
  (bind _asbp_ps_team_state_crp (Utilities|Casting|CastToBP_PS_TeamState_CRP (Utilities|Array|Get(acopy) (Variables|/Script/Squad.SQGameState|GetIndexedTeamStates _aspsgame_state) (Utilities|Select :Index (Variables|Default|GetZombieTeamId) :Option%200 0 :Option%201 2 :Option%202 1))))
  (Default|ReCalculateSquadLimits _asbp_ps_team_state_crp))

(fn ConstructionScript
  (|CallParentFunction))

(fn AllowTeamChangeBP
  (params (RequestingPlayer :type SQ%20Player%20Controller%20Object%20Reference) (NewTeam :type Integer))
  (bind _asbp_player_state_crp (Utilities|Casting|CastToBP_PlayerState_CRP (Variables|/Script/Engine.Controller|GetPlayerState RequestingPlayer))
    (:then
      (bind _asbp_game_state_crp (Utilities|Casting|CastToBP_GameState_CRP (Game|GetGameState))
        (:then
          (if (== NewTeam (Variables|Default|GetZombieTeamId))
            ;[1 1 1] no restriction on joining zombies
            (return true)
            (else
              (bind _asbp_ps_player_controller (Utilities|Casting|CastToBP_PS_PlayerController RequestingPlayer))
              ;[1 1 1] already died as a suvivor?
              (if (Utilities|Array|ContainsItem (Variables|/Community_Resource_Pack/Gameplay/Gamemodes/CRPMain/BP_GameState_CRP.BP_GameState_CRP_C|GetDeadPlayers _asbp_game_state_crp) (Class|SQPlayerState|GetUniqueNetID _asbp_player_state_crp))
                (Class|SQPlayerController|ClientShowToast _asbp_ps_player_controller (Utilities|Text|MakeLiteralText "You failed to survive, you cannot join the survivors") 5.0)
                (return false)
                (else
                  ;[1 1 1] cut off time reached?
                  (if (> (- (Variables|Default|GetRoundTime) (Class|SQGameState|GetRemainingTime _asbp_game_state_crp)) (Variables|Default|GetSurvivorTeamChangeLockTime))
                    (Class|SQPlayerController|ClientShowToast _asbp_ps_player_controller (Utilities|Text|MakeLiteralText "7 minutes have passed, Survivors have been cut off") 5.0)
                    (return false)
                    (else
                      (return true))))))))
        (:CastFailed
          _)))
    (:CastFailed
      _))
  (bind _returnvalue (|CallParentFunction RequestingPlayer NewTeam))
  (return _returnvalue))

(fn GetConcretePawnClassforController
  (params (InController :type Controller%20Object%20Reference))
  (bind _asbp_player_state_crp (Utilities|Casting|CastToBP_PlayerState_CRP (Variables|/Script/Engine.Controller|GetPlayerState InController))
    (:then
      (if (Variables|/Community_Resource_Pack/Gameplay/Gamemodes/CRPMain/BP_PlayerState_CRP.BP_PlayerState_CRP_C|GetbSurvivorKilledByZombie _asbp_player_state_crp)
        (return (Variables|/Community_Resource_Pack/Gameplay/Gamemodes/CRPMain/BP_PlayerState_CRP.BP_PlayerState_CRP_C|GetSurvivorCharacterClass _asbp_player_state_crp))
        (else
          _)))
    (:CastFailed
      _))
  (bind _returnvalue (|CallParentFunction InController))
  (return _returnvalue))

(fn FindPlayerStart
  (params (Player :type Controller%20Object%20Reference) (IncomingName :type String))
  (bind _asbp_player_state_crp (Utilities|Casting|CastToBP_PlayerState_CRP (Variables|/Script/Engine.Controller|GetPlayerState Player))
    (:then
      (if (Variables|/Community_Resource_Pack/Gameplay/Gamemodes/CRPMain/BP_PlayerState_CRP.BP_PlayerState_CRP_C|GetbSurvivorKilledByZombie _asbp_player_state_crp)
        (return (Variables|/Community_Resource_Pack/Gameplay/Gamemodes/CRPMain/BP_PlayerState_CRP.BP_PlayerState_CRP_C|GetSurvivorZombieRevivePoint _asbp_player_state_crp))
        (else
          _)))
    (:CastFailed
      _))
  (bind _returnvalue (|CallParentFunction Player IncomingName))
  (return _returnvalue))

(fn PlayerCanRestart
  (params (Player :type Player%20Controller%20Object%20Reference))
  (bind _asbp_player_state_crp (Utilities|Casting|CastToBP_PlayerState_CRP (Variables|/Script/Engine.Controller|GetPlayerState Player))
    (:then
      (if (Variables|/Community_Resource_Pack/Gameplay/Gamemodes/CRPMain/BP_PlayerState_CRP.BP_PlayerState_CRP_C|GetbShouldSpawn _asbp_player_state_crp)
        (if (!= (Variables|/Script/Squad.SQTeamState|GetId (Class|SQPlayerState|GetTeamState _asbp_player_state_crp)) (Variables|Default|GetZombieTeamId))
          (if (and (Utilities|IsValid (Variables|/Script/Squad.SQPlayerState|GetSquadState _asbp_player_state_crp)) (Utilities|IsValid (Class|SQPlayerController|GetSelectedSpawn (.AsPSPlayer%20Controller (Utilities|Casting|CastToPSPlayerController Player)))))
            _
            (else
              (bind _aspsplayer_controller (Utilities|Casting|CastToPSPlayerController Player))
              (Class|SQPlayerController|ClientShowToast _aspsplayer_controller (Utilities|Text|MakeLiteralText "You need to be in a squad to spawn as a survivor") 5.0)
              (return false))))
        (else
          (return false))))
    (:CastFailed
      _))
  (bind _returnvalue (|CallParentFunction Player))
  (return _returnvalue))

(fn ChooseTeamBP
  (params (ForPC :type SQ%20Player%20Controller%20Object%20Reference))
  (bind _asbp_game_state_crp (Utilities|Casting|CastToBP_GameState_CRP (Game|GetGameState)))
  ;[1 1 1] cut off time reached?
  (if (> (- (Variables|Default|GetRoundTime) (Class|SQGameState|GetRemainingTime _asbp_game_state_crp)) (Variables|Default|GetSurvivorTeamChangeLockTime))
    _
    (else
      (bind _assqplayer_state (Utilities|Casting|CastToSQPlayerState (Variables|/Script/Engine.Controller|GetPlayerState ForPC)))
      ;[1 1 1] already died as survivor
      (if (Utilities|Array|ContainsItem (Variables|/Community_Resource_Pack/Gameplay/Gamemodes/CRPMain/BP_GameState_CRP.BP_GameState_CRP_C|GetDeadPlayers _asbp_game_state_crp) (Class|SQPlayerState|GetUniqueNetID _assqplayer_state))
        _
        (else
          (bind _returnvalue (|CallParentFunction ForPC))
          (return _returnvalue)))))
  (return (Variables|/Script/Squad.SQTeamState|GetAuthorityTeam (Utilities|Array|Get(acopy) (Variables|/Script/Squad.SQGameState|GetIndexedTeamStates _asbp_game_state_crp) (Variables|Default|GetZombieTeamId)))))
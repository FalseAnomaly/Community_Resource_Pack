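; Child Blueprint of a RAAS lattice class, apparently for a RAAS gamemode variant, that adds almost no logic of its own.
; Its construction script and its FOB placement and dynamic spawn location checks simply pass through to the parent.
; The FOB overlay drawing override returns without calling the parent or supplying any instructions.
; Overlap and Tick events are disabled placeholder nodes.
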(event Collision|EventActorBeginOverlap
  (params (OtherActor :type Actor%20Object%20Reference))
  (|CallParentFunction OtherActor) ; This node is disabled and will not be called.\nDrag off pins to build functionality.
)

(event EventTick
  (params (DeltaSeconds :type Float%20%28single-precision%29))
  (|CallParentFunction DeltaSeconds) ; This node is disabled and will not be called.\nDrag off pins to build functionality.
)

(fn ConstructionScript
  (|CallParentFunction))

(fn GetFOBOverlayDrawingInstructions
  (return 0))

(fn IsFOBPlacementValid
  (params (Location :type Vector :default "0, 0, 0"))
  (bind _valid (|CallParentFunction Location))
  (return _valid))

(fn IsDynamicSpawnLocationValidLocation
  (params (Location :type Vector :default "0, 0, 0") (ForTeam :type ESQTeam%20Enum :default "Team_Neutral"))
  (bind _bplacementvalid (|CallParentFunction Location ForTeam))
  (return _bplacementvalid))
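; Game mode Blueprint for a RAAS child variant that can create a squad tied to an armored on-demand vehicle spawner.
; CreateSquadFor resolves the given team to its PSTeam and creates a blank squad using the spawner's squad name and intended section, sized to the vehicle's seat count.
; BeginPlay and construction only call the parent, and Tick is disabled.
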(event EventBeginPlay
  (|CallParentFunction))

(event EventTick
  (params (DeltaSeconds :type Float%20%28single-precision%29))
  (|CallParentFunction DeltaSeconds) ; This node is disabled and will not be called.\nDrag off pins to build functionality.
)

(fn ConstructionScript
  (|CallParentFunction))

(fn CreateSquadfor
  (params (VehicleSpawner :type SQ%20Vehicle%20Spawner%20Object%20Reference) (Team :type ESQTeam%20Enum :default "Team_Neutral"))
  (bind _asbp_armored_on_demand_vehicle_spawner (Utilities|Casting|CastToBP_ArmoredOnDemandVehicleSpawner VehicleSpawner))
  (bind _aspsteam (Utilities|Casting|CastToPSTeam (Utilities|Array|Get(acopy) (Variables|Default|GetIndexedTeams) (Utilities|Select :Index Team :Team_Neutral 0 :Team_One 1 :Team_Two 2))))
  (Class|PSTeam|CreateBlankPSSquad _aspsteam (Variables|/Game/Gameplay/BP_ArmoredOnDemandVehicleSpawner.BP_ArmoredOnDemandVehicleSpawner_C|GetSquadName _asbp_armored_on_demand_vehicle_spawner) (Variables|/Game/Gameplay/BP_ArmoredOnDemandVehicleSpawner.BP_ArmoredOnDemandVehicleSpawner_C|GetIntendedSection _asbp_armored_on_demand_vehicle_spawner) (Default|GetVehicleSeatCount _asbp_armored_on_demand_vehicle_spawner)))
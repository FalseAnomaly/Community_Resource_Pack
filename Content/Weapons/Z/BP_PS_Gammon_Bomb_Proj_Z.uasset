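; Gammon bomb throwable projectile that detonates on impact, provided it has flown long enough first.
; On the first hit after a minimum flight time it runs parent impact logic, then calls Explode and force-detonates the throwable explosive component, a noted hack for vehicle damage and fuses.
; An earlier hit uses up the first-hit flag, disabling impact detonation.
; Tick tracks flight time and spins the mesh until it slows down.
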(event EventOnImpact
  (params (SelfActor :type Actor%20Object%20Reference) (OtherActor :type Actor%20Object%20Reference) (NormalImpulse :type Vector :default "0, 0, 0") (Hit :type Hit%20Result%20Structure%20%28by%20ref%29))
  (Variables|Default|SetLastImpactHitResult Hit)
  (if (and (>= (Variables|Default|GetFlightTime) (Variables|Default|GetMinFlightTime)) (Variables|Default|GetIsFirstHit))
    (Variables|Default|SetIsFirstHit false)
    (Variables|Default|SetLastImpactNormal (.Normal (Collision|BreakHitResult Hit)))
    (|CallParentFunction SelfActor OtherActor NormalImpulse Hit)
    ;[1 1 1] Hack for vehicle damage and fuses
    (CallFunction|Explode)
    (Class|PSExplosiveComponent|Detonate (Variables|Default|GetPSExplosiveComponentThrowable) self 0 true)
    (else
      (Variables|Default|SetIsFirstHit false))))

(event EventTick
  (params (DeltaSeconds :type Float%20%28single-precision%29))
  (|CallParentFunction DeltaSeconds)
  (Variables|Default|SetFlightTime (+ DeltaSeconds (Variables|Default|GetFlightTime)))
  (if (Variables|Default|GetKeepRotating)
    (Transformation|AddLocalRotation (Variables|Default|GetProjectileMesh) (Math|Rotator|MakeRotator 0.0 (* DeltaSeconds (Variables|Default|GetRotationSpeed)) 0.0) false false)
    (Variables|Default|SetKeepRotating (> (Math|Vector|VectorLength (Transformation|GetVelocity)) 1e+02))))

(fn ConstructionScript
  (|CallParentFunction))
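; Zombie melee weapon Blueprint that adds hit handling against explosive deployables and M3 actors when it fires.
; After the parent fire logic, it line traces on Visibility from the fire origin along the owning soldier's aim, out to the trace distance.
; The authority applies melee damage to those targets, with a different amount and damage type for each.
; Remote instances only play the target's damage FX at the impact point.
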(event EventBlueprintonFire
  (params (Origin :type Vector%20%28by%20ref%29 :default "0, 0, 0"))
  (bind _returnvalue (Class|SQInfantryWeapon|GetOwnerSoldier))
  (bind _returnvalue_2 (Pawn|GetController _returnvalue))
  (|CallParentFunction Origin)
  (bind _outhit (Collision|LineTraceByChannel Origin (+ Origin (* (Math|Rotator|GetRotationXVector (Pawn|GetBaseAimRotation (Class|SQInfantryWeapon|GetOwnerSoldier))) (Variables|Default|GetTraceDistance))) "TraceTypeQuery1" false 0 "None"))
  (Networking|SwitchHasAuthority
    (:Authority
      (Utilities|FlowControl|Sequence
        (:then_0
          (bind _asbp_psdeployable_explosive_z (Utilities|Casting|CastToBP_PSDeployable_Explosive_Z (.HitActor (Collision|BreakHitResult _outhit))))
          (Game|Damage|ApplyDamage _asbp_psdeployable_explosive_z 1e+02 _returnvalue_2 _returnvalue "/Game/Gameplay/DamageTypes/BP_Melee.BP_Melee_C"))
        (:then_1
          (bind _asbp_m3_z (Utilities|Casting|CastToBP_M3_Z (.HitActor (Collision|BreakHitResult _outhit))))
          (Game|Damage|ApplyDamage _asbp_m3_z 1e+01 _returnvalue_2 _returnvalue "/Community_Resource_Pack/Gameplay/DamageTypes/BP_Melee_Z.BP_Melee_Z_C"))))
    (:Remote
      (Utilities|FlowControl|Sequence
        (:then_0
          (bind _asbp_psdeployable_explosive_z_2 (Utilities|Casting|CastToBP_PSDeployable_Explosive_Z (.HitActor (Collision|BreakHitResult _outhit))))
          (Default|DoDamageFX _asbp_psdeployable_explosive_z_2 (.ImpactPoint (Collision|BreakHitResult _outhit))))
        (:then_1
          (bind _asbp_m3_z_2 (Utilities|Casting|CastToBP_M3_Z (.HitActor (Collision|BreakHitResult _outhit))))
          (Default|DoDamageFX _asbp_m3_z_2 (.ImpactPoint (Collision|BreakHitResult _outhit))))))))

(fn ConstructionScript
  (|CallParentFunction))
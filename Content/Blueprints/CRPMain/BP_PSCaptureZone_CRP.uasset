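; CRP child of the PS capture zone that sets whether its capture zone component uses RAAS and Armored behavior.
; BeginPlay retries every second until the game state and its GameMode class are valid, applying these flags before calling parent BeginPlay.
; Each flag defaults to whether the game mode is of that type.
; A game state implementing InterfaceCRP can force either flag on or off.
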(event Custom|OverrideComponentSettings
  (bind _returnvalue (Game|GetGameState))
  (bind _bp_pscapturezonecomponent (Variables|Default|GetBP_PSCaptureZoneComponent))
  (bind _gamemodeclass (Variables|/Script/Engine.GameStateBase|GetGameModeClass _returnvalue))
  (if (Utilities|DoesObjectImplementInterface _returnvalue (Variables|Default|GetInterfaceCRP))
    (bind _return_value (Class|BPIGameStateCRP|UseRAASFeatures(Message) _returnvalue))
    (Utilities|Casting|CastToBP_GameMode_PS_RAASClass _gamemodeclass
      (:then
        (Variables|/Game/PostScriptum/Blueprints/BP_PSCaptureZoneComponent.BP_PSCaptureZoneComponent_C|SetbIsRAAS _bp_pscapturezonecomponent (!= _return_value 2)))
      (:CastFailed
        (Variables|/Game/PostScriptum/Blueprints/BP_PSCaptureZoneComponent.BP_PSCaptureZoneComponent_C|SetbIsRAAS _bp_pscapturezonecomponent (== _return_value 1))))
    (bind _return_value_2 (Class|BPIGameStateCRP|UseVanillaArmoredFeatures(Message) _returnvalue))
    (Utilities|Casting|CastToBP_PS_GameMode_ArmoredClass _gamemodeclass
      (:then
        (Variables|/Game/PostScriptum/Blueprints/BP_PSCaptureZoneComponent.BP_PSCaptureZoneComponent_C|SetbIsArmored _bp_pscapturezonecomponent (!= _return_value_2 2)))
      (:CastFailed
        (Variables|/Game/PostScriptum/Blueprints/BP_PSCaptureZoneComponent.BP_PSCaptureZoneComponent_C|SetbIsArmored _bp_pscapturezonecomponent (== _return_value_2 1))))
    (else
      (Utilities|Casting|CastToBP_GameMode_PS_RAASClass _gamemodeclass
        (:then
          (Variables|/Game/PostScriptum/Blueprints/BP_PSCaptureZoneComponent.BP_PSCaptureZoneComponent_C|SetbIsRAAS _bp_pscapturezonecomponent true))
        (:CastFailed
          (Variables|/Game/PostScriptum/Blueprints/BP_PSCaptureZoneComponent.BP_PSCaptureZoneComponent_C|SetbIsRAAS _bp_pscapturezonecomponent false)))
      (Utilities|Casting|CastToBP_PS_GameMode_ArmoredClass _gamemodeclass
        (:then
          (Variables|/Game/PostScriptum/Blueprints/BP_PSCaptureZoneComponent.BP_PSCaptureZoneComponent_C|SetbIsArmored _bp_pscapturezonecomponent true))
        (:CastFailed
          (Variables|/Game/PostScriptum/Blueprints/BP_PSCaptureZoneComponent.BP_PSCaptureZoneComponent_C|SetbIsArmored _bp_pscapturezonecomponent false))))))

(event EventBeginPlay
  (bind _returnvalue (Game|GetGameState))
  (Utilities|Casting|CastToBP_GameState _returnvalue :!label _label
    (:then
      (if (Utilities|IsValidClass (Variables|/Script/Engine.GameStateBase|GetGameModeClass _returnvalue)) :!label _label_2
        (CallFunction|OverrideComponentSettings)
        (|CallParentFunction)
        (else
          (Utilities|FlowControl|Delay 1.0)
          (goto _label_2))))
    (:CastFailed
      (Utilities|FlowControl|Delay 1.0)
      (goto _label))))

(event Collision|EventActorBeginOverlap
  (params (OtherActor :type Actor%20Object%20Reference)))

(event EventTick
  (params (DeltaSeconds :type Float%20%28single-precision%29)))

(fn ConstructionScript
  (|CallParentFunction))
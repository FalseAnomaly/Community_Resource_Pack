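; Carried ammo crate item that slows its soldier and is loaded into a nearby BP_ObjectiveLoad_Z truck.
; Holding use runs a timed progress bar, then adds the crate via a sphere-overlap truck search and signals the game state.
; The server attaches an objective marker to the carrier and polls for vehicle entry.
; Entering a vehicle, dying or switching items unplaced drops a BP_AmmoBagPickup_Z at a traced location.
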(event Custom|CustomEvent_0
  (params (StaticInfo :type SQ%20Item%20Static%20Info%20Object%20Reference))
  (if (!= StaticInfo (Class|SQEquipableItem|GetItemStaticInfo))
    (CallFunction|UnequippedonClient)))

(event Custom|onPlaced
  (Variables|Default|SetbPlaced true))

(event Custom|CustomEvent_1
  (bind _markerhelper (Variables|Default|GetMarkerHelper))
  (bind _asbp_ps_mutable_soldier (Utilities|Casting|CastToBP_PS_MutableSoldier (Class|SQEquipableItem|GetOwnerPawn)))
  (if (Class|SQSoldier|IsinVehicle _asbp_ps_mutable_soldier)
    (Variables|Default|SetbPlaced true)
    (Variables|Default|SetItemCount self 0)
    (CallFunction|DropSelffromVehicle)
    (Utilities|IsValid _markerhelper
      (:Is%20Valid
        (Actor|DestroyActor _markerhelper)))))

(event Custom|CustomEvent_2
  (CallFunction|CustomEvent1))

(event Custom|OnSoldierDied_Event_0
  (params (DeadSoldier :type PS%20Soldier%20Object%20Reference) (Killer :type Pawn%20Object%20Reference) (DamageCauser :type Actor%20Object%20Reference) (bPointDamage :type Boolean))
  (bind _markerhelper (Variables|Default|GetMarkerHelper))
  (if (Variables|Default|GetbPlaced)
    _
    (else
      (CallFunction|DropSelf)))
  (Utilities|IsValid _markerhelper
    (:Is%20Valid
      (Actor|DestroyActor _markerhelper))))

(event Custom|TryLoading
  (params (Loader :type SQ%20Player%20Controller%20Object%20Reference))
  (bind _vehiclecheckerhandle (Variables|Default|GetVehicleCheckerHandle))
  (bind _loadingradius (Variables|Default|GetLoadingRadius))
  (bind _markerhelper (Variables|Default|GetMarkerHelper))
  (bind (_truckload _bfound) (CallFunction|FindTruck _loadingradius))
  (if _bfound
    (Default|AddItemtoTruck _truckload)
    (Variables|Default|SetbPlaced true)
    (bind _aspssoldier (Utilities|Casting|CastToPSSoldier (Class|SQEquipableItem|GetOwnerPawn)))
    (Class|SQPawnInventoryComponent|SwitchItem (Variables|/Script/Squad.SQSoldier|GetInventoryComponent _aspssoldier))
    (bind _asbp_game_state_crp (Utilities|Casting|CastToBP_GameState_CRP (Game|GetGameState)))
    (Default|SignalImportantEvent _asbp_game_state_crp 1.0)
    (Utilities|IsValid _markerhelper
      (:Is%20Valid
        (Actor|DestroyActor _markerhelper)
        (if (Utilities|Time|IsValidTimerHandle _vehiclecheckerhandle)
          (Utilities|Time|ClearandInvalidateTimerbyHandle _vehiclecheckerhandle))))
    (else
      (Class|SQPlayerController|ShowToast Loader (Variables|Default|GetNoTruckAvailableText) 5.0 false))))

(event Custom|UnequippedOnClient
  (bind _markerhelper (Variables|Default|GetMarkerHelper))
  (bind _asbp_ps_mutable_soldier (Utilities|Casting|CastToBP_PS_MutableSoldier (Class|SQEquipableItem|GetOwnerPawn)))
  (Class|SQPawnInventoryComponent|RemoveItemfromInventory (Class|SQSoldier|GetInventory _asbp_ps_mutable_soldier))
  (if (Variables|Default|GetbPlaced)
    _
    (else
      (CallFunction|DropSelf)))
  (Utilities|IsValid _markerhelper
    (:Is%20Valid
      (Actor|DestroyActor _markerhelper))))

(event Custom|LoadingTimer
  (CallFunction|TryLoading (Variables|Default|GetLoadingController)))

(event EventOnSoldierDeath
  (|CallParentFunction)
  (Rendering|SetVisibility (Variables|Default|GetMesh1P) false true))

(event EventBlueprintonEquip
  (|CallParentFunction)
  (bind _asbp_ps_mutable_soldier (Utilities|Casting|CastToBP_PS_MutableSoldier (Class|SQEquipableItem|GetOwnerPawn)))
  (bind _assqsoldier_movement (Utilities|Casting|CastToSQSoldierMovement (Variables|/Script/Engine.Character|GetCharacterMovement _asbp_ps_mutable_soldier)))
  (Variables|/Script/Engine.CharacterMovementComponent|SetMaxWalkSpeed (Variables|/Script/Engine.Character|GetCharacterMovement _asbp_ps_mutable_soldier) 2e+02)
  (Variables|/Script/Engine.CharacterMovementComponent|SetMaxWalkSpeedCrouched _assqsoldier_movement 1e+02)
  (Variables|/Script/Squad.SQSoldierMovement|SetMaxWalkSpeedProne _assqsoldier_movement 75.0))

(event EventBeginPlay
  (|CallParentFunction)
  (Networking|SwitchHasAuthority
    (:Authority
      (EventDispatchers|BindEventtoItemPlacedReal (delegate Custom|onPlaced))
      (bind _asbp_ps_mutable_soldier (Utilities|Casting|CastToBP_PS_MutableSoldier (Class|SQEquipableItem|GetOwnerPawn)))
      (EventDispatchers|AssignOnSoldierDied _asbp_ps_mutable_soldier (delegate Custom|OnSoldierDied_Event_0))
      (bind _returnvalue (Game|SpawnActorfromClass "/Game/PostScriptum/Gameplay/Halloween/TruckInvasion/Items/BP_HalloweenObjetiveMarkerHelper.BP_HalloweenObjetiveMarkerHelper_C" (Transformation|GetActorTransform) "AlwaysSpawn" 0 0))
      (bind _output_get (Variables|Default|SetMarkerHelper _returnvalue))
      (Transformation|AttachActorToActor _output_get (Class|SQEquipableItem|GetOwnerPawn) "None" "SnapToTarget" "SnapToTarget" "SnapToTarget" true)
      (bind _returnvalue_2 (Utilities|Time|SetTimerbyEvent (delegate Custom|CustomEvent_2) 0.5 true))
      (Variables|Default|SetVehicleCheckerHandle _returnvalue_2))
    (:Remote
      (bind _asbp_ps_mutable_soldier_2 (Utilities|Casting|CastToBP_PS_MutableSoldier (Class|SQEquipableItem|GetOwnerPawn)))
      (EventDispatchers|BindEventtoEquippedNewItemEvent (Class|SQSoldier|GetInventory _asbp_ps_mutable_soldier_2) (delegate Custom|CustomEvent_0)))))

(event EventBPEndUse
  (if (Pawn|IsLocallyControlled (Class|SQEquipableItem|GetOwnerPawn))
    (Utilities|Time|ClearandInvalidateTimerbyHandle (Variables|Default|GetLoadingTimerHandle))
    (bind _asbp_ps_hud (Utilities|Casting|CastToBP_PS_HUD (HUD|GetHUD (Variables|Default|GetLoadingController))))
    (Default|CancelProgressBar _asbp_ps_hud)))

(event EventBPonUsed
  (params (User :type Controller%20Object%20Reference))
  (bind _loadingtime (Variables|Default|GetLoadingTime))
  (if (== (Pawn|GetController (Class|SQEquipableItem|GetOwnerPawn)) User)
    (bind _asbp_ps_player_controller (Utilities|Casting|CastToBP_PS_PlayerController User))
    (Variables|Default|SetLoadingController _asbp_ps_player_controller)
    (bind _asbp_ps_hud (Utilities|Casting|CastToBP_PS_HUD (HUD|GetHUD (Variables|Default|GetLoadingController))))
    (if (.bFound (CallFunction|FindTruck (Variables|Default|GetLoadingRadius)))
      (Default|StartProgressBar _asbp_ps_hud _loadingtime "/Game/UI/Widgets/HUD/Scoreboard/ScoreboardTextures/ScoreboardArrow.ScoreboardArrow")
      (bind _returnvalue (Utilities|Time|SetTimerbyEvent (delegate Custom|LoadingTimer) _loadingtime))
      (Variables|Default|SetLoadingTimerHandle _returnvalue)
      (Class|SQPlayerController|ShowToast (Variables|Default|GetLoadingController) (Utilities|Text|MakeLiteralText "Loading crate into truck") 5.0 false)
      (else
        (Class|SQPlayerController|ShowToast (Variables|Default|GetLoadingController) (Variables|Default|GetNoTruckAvailableText) 5.0 false)))))

(event EventBlueprintonEquipped
  (|CallParentFunction))

(event EventBlueprintonUnequipped
  (|CallParentFunction)
  (bind _asbp_ps_mutable_soldier (Utilities|Casting|CastToBP_PS_MutableSoldier (Class|SQEquipableItem|GetOwnerPawn)))
  (bind _assqsoldier_movement (Utilities|Casting|CastToSQSoldierMovement (Variables|/Script/Engine.Character|GetCharacterMovement _asbp_ps_mutable_soldier)))
  (Variables|/Script/Engine.CharacterMovementComponent|SetMaxWalkSpeed _assqsoldier_movement (Variables|Default|GetDefaultWalkSpeed))
  (Variables|/Script/Engine.CharacterMovementComponent|SetMaxWalkSpeedCrouched _assqsoldier_movement (Variables|Default|GetdefaultCrouchSpeed))
  (Variables|/Script/Squad.SQSoldierMovement|SetMaxWalkSpeedProne _assqsoldier_movement (Variables|Default|GetDefaultProneSpeed)))

(event EventBPStopUsed
  (params (User :type Controller%20Object%20Reference))
  (if (== User (Variables|Default|GetLoadingController))
    (Utilities|Time|ClearandInvalidateTimerbyHandle (Variables|Default|GetLoadingTimerHandle))
    (bind _asbp_ps_hud (Utilities|Casting|CastToBP_PS_HUD (HUD|GetHUD (Variables|Default|GetLoadingController))))
    (Default|CancelProgressBar _asbp_ps_hud)))

(event EventBPBeginUse
  (bind _returnvalue (Class|SQEquipableItem|GetOwnerPawn))
  (bind _loadingtime (Variables|Default|GetLoadingTime))
  (if (Pawn|IsLocallyControlled _returnvalue)
    (bind _asbp_ps_player_controller (Utilities|Casting|CastToBP_PS_PlayerController (Pawn|GetController _returnvalue)))
    (Variables|Default|SetLoadingController _asbp_ps_player_controller)
    (bind _asbp_ps_hud (Utilities|Casting|CastToBP_PS_HUD (HUD|GetHUD (Variables|Default|GetLoadingController))))
    (if (.bFound (CallFunction|FindTruck (Variables|Default|GetLoadingRadius)))
      (Default|StartProgressBar _asbp_ps_hud _loadingtime "/Game/UI/Widgets/HUD/Scoreboard/ScoreboardTextures/ScoreboardArrow.ScoreboardArrow")
      (bind _returnvalue_2 (Utilities|Time|SetTimerbyEvent (delegate Custom|LoadingTimer) _loadingtime))
      (Variables|Default|SetLoadingTimerHandle _returnvalue_2)
      (Class|SQPlayerController|ShowToast (Variables|Default|GetLoadingController) (Utilities|Text|MakeLiteralText "Loading crate into truck") 5.0 false)
      (else
        (Class|SQPlayerController|ShowToast (Variables|Default|GetLoadingController) (Variables|Default|GetNoTruckAvailableText) 5.0 false)))))

(fn ConstructionScript
  (|CallParentFunction))

(fn DropSelf
  (bind _returnvalue (Class|SQEquipableItem|GetOwnerPawn))
  (bind _vehiclecheckerhandle (Variables|Default|GetVehicleCheckerHandle))
  (bind _returnvalue_2 (Transformation|GetActorLocation _returnvalue))
  (bind (_x _y _z) (Math|Vector|BreakVector _returnvalue_2))
  (bind _outhit (Collision|LineTraceForObjects _returnvalue_2 (Math|Vector|MakeVector _x _y (- _z 1e+02)) (Utilities|Array|MakeArray "ObjectTypeQuery1") false 0 "ForDuration"))
  (bind _returnvalue_3 (Game|SpawnActorfromClass "/Community_Resource_Pack/Blueprints/Z/BP_AmmoBagPickup_Z.BP_AmmoBagPickup_Z_C" (Math|Transform|MakeTransform (+ (select (.bBlockingHit (Collision|BreakHitResult _outhit)) (.ImpactPoint (Collision|BreakHitResult _outhit)) (.TraceEnd (Collision|BreakHitResult _outhit))) (* (Transformation|GetActorForwardVector _returnvalue) 1.5e+02))) "AlwaysSpawn" 0 false (Utilities|GetClass self) true true 0))
  (Transformation|SetActorScale3D _returnvalue_3 "1.800000,1.800000,1.800000")
  (if (Utilities|Time|IsValidTimerHandle _vehiclecheckerhandle)
    (Utilities|Time|ClearandInvalidateTimerbyHandle _vehiclecheckerhandle))
  (return _returnvalue_3))

(fn OnRepMarkerHelper)

(fn FindTruck
  (params (WithinRadius :type Float%20%28single-precision%29))
  (bind (_outactors _returnvalue) (Collision|SphereOverlapActors (Transformation|GetActorLocation) WithinRadius (Utilities|Array|MakeArray "ObjectTypeQuery2" "ObjectTypeQuery1") "/Community_Resource_Pack/Blueprints/Z/BP_ObjectiveLoad_Z.BP_ObjectiveLoad_Z_C"))
  (if _returnvalue
    (bind _asbp_objective_load_z (Utilities|Casting|CastToBP_ObjectiveLoad_Z (Utilities|Array|Get(acopy) _outactors))
      (:then
        (return _asbp_objective_load_z true))
      (:CastFailed
        _)))
  (return 0 false))

(fn DropSelffromVehicle
  (bind _vehiclecheckerhandle (Variables|Default|GetVehicleCheckerHandle))
  (bind _asbp_ps_mutable_soldier (Utilities|Casting|CastToBP_PS_MutableSoldier (Class|SQEquipableItem|GetOwnerPawn)))
  (Utilities|IsValid (Class|SQSoldier|GetCurrentVehicle _asbp_ps_mutable_soldier)
    (:Is%20Valid
      (bind _outhit (Collision|LineTraceForObjects (Transformation|GetActorLocation (Class|SQSoldier|GetCurrentVehicle _asbp_ps_mutable_soldier)) (Math|Vector|MakeVector (.X (Math|Vector|BreakVector (Transformation|GetActorLocation (Class|SQSoldier|GetCurrentVehicle _asbp_ps_mutable_soldier)))) (.Y (Math|Vector|BreakVector (Transformation|GetActorLocation (Class|SQSoldier|GetCurrentVehicle _asbp_ps_mutable_soldier)))) (- (.Z (Math|Vector|BreakVector (Transformation|GetActorLocation (Class|SQSoldier|GetCurrentVehicle _asbp_ps_mutable_soldier)))) 0.0)) (Utilities|Array|MakeArray "ObjectTypeQuery1") false 0 "ForDuration"))
      (bind _returnvalue (Game|SpawnActorfromClass "/Community_Resource_Pack/Blueprints/Z/BP_AmmoBagPickup_Z.BP_AmmoBagPickup_Z_C" (Math|Transform|MakeTransform (+ (select (.bBlockingHit (Collision|BreakHitResult _outhit)) (.ImpactPoint (Collision|BreakHitResult _outhit)) (.TraceEnd (Collision|BreakHitResult _outhit))) (* (Transformation|GetActorForwardVector (Class|SQSoldier|GetCurrentVehicle _asbp_ps_mutable_soldier)) 1.5e+02))) "AlwaysSpawn" 0 false (Utilities|GetClass self) true true 0))
      (if (Utilities|Time|IsValidTimerHandle _vehiclecheckerhandle)
        (Utilities|Time|ClearandInvalidateTimerbyHandle _vehiclecheckerhandle))
      (return _returnvalue))
    (:Is%20Not%20Valid
      (CallFunction|DropSelf))))

(fn GetInterfaceTeam
  (return 0))

(fn GetUsableData
  (return ""))
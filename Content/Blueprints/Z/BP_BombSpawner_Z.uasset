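; Bomb build site that lets players turn a fully loaded supply truck into a deployable explosive and extra match time.
; Its sphere tracks an overlapping vehicle's load, updating CanBuild and turning the bomb meshes glowing green when full.
; TryActivating spawns the explosive, empties the truck, toasts all players, adds three minutes through an authority-only admin console command and destroys itself.
; Failed attempts toast the player the reason.
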(event OnComponentBeginOverlap(Sphere)
  (params (OverlappedComponent :type Primitive%20Component%20Object%20Reference) (OtherActor :type Actor%20Object%20Reference) (OtherComp :type Primitive%20Component%20Object%20Reference) (OtherBodyIndex :type Integer) (bFromSweep :type Boolean) (SweepResult :type Hit%20Result%20Structure%20%28by%20ref%29))
  (bind _ju87_bomb (Variables|Default|GetJu87_Bomb))
  (bind _staticmesh (Variables|Default|GetStaticMesh))
  (bind _asbpi_zombie_load_vehicle_z (Utilities|Casting|CastToBPI_ZombieLoadVehicle_Z OtherActor))
  (bind _loadactor (Default|GetLoadActor _asbpi_zombie_load_vehicle_z))
  (EventDispatchers|BindEventtoOnTruckLoadChanged _loadactor (delegate Custom|TruckLoadChanged))
  (bind _output_get (Variables|Default|SetMyLoad _loadactor))
  (bind _output_get_2 (Variables|Default|SetbCanBuild (.Filled (Default|IsCompletelyFilled _output_get))))
  (for _index (range 0 (- (Rendering|Material|GetNumMaterials _ju87_bomb) 1))
    (Rendering|Material|SetMaterial _ju87_bomb _index (select _output_get_2 "/Game/PostScriptum/Gameplay/Halloween/M_GlowingMaterial_Inst_Green.M_GlowingMaterial_Inst_Green" "/Game/PostScriptum/Gameplay/Halloween/M_GlowingMaterial.M_GlowingMaterial")))
  (for _index_2 (range 0 (- (Rendering|Material|GetNumMaterials _staticmesh) 1))
    (Rendering|Material|SetMaterial _staticmesh _index_2 (select _output_get_2 "/Game/PostScriptum/Gameplay/Halloween/M_GlowingMaterial_Inst_Green.M_GlowingMaterial_Inst_Green" "/Game/PostScriptum/Gameplay/Halloween/M_GlowingMaterial.M_GlowingMaterial"))))

(event OnComponentEndOverlap(Sphere)
  (params (OverlappedComponent :type Primitive%20Component%20Object%20Reference) (OtherActor :type Actor%20Object%20Reference) (OtherComp :type Primitive%20Component%20Object%20Reference) (OtherBodyIndex :type Integer))
  (bind _ju87_bomb (Variables|Default|GetJu87_Bomb))
  (bind _staticmesh (Variables|Default|GetStaticMesh))
  (bind _asbpi_zombie_load_vehicle_z (Utilities|Casting|CastToBPI_ZombieLoadVehicle_Z OtherActor))
  (bind _loadactor (Default|GetLoadActor _asbpi_zombie_load_vehicle_z))
  (EventDispatchers|UnbindEventfromOnTruckLoadChanged _loadactor (delegate Custom|TruckLoadChanged))
  (Variables|Default|SetbCanBuild false)
  (Variables|Default|SetMyLoad 0)
  (for _index (range 0 (- (Rendering|Material|GetNumMaterials _ju87_bomb) 1))
    (Rendering|Material|SetMaterial _ju87_bomb _index (select (stale OnComponentBeginOverlap(Sphere) _output_get_2) "/Game/PostScriptum/Gameplay/Halloween/M_GlowingMaterial_Inst_Green.M_GlowingMaterial_Inst_Green" "/Game/PostScriptum/Gameplay/Halloween/M_GlowingMaterial.M_GlowingMaterial")))
  (for _index_2 (range 0 (- (Rendering|Material|GetNumMaterials _staticmesh) 1))
    (Rendering|Material|SetMaterial _staticmesh _index_2 (select (stale OnComponentBeginOverlap(Sphere) _output_get_2) "/Game/PostScriptum/Gameplay/Halloween/M_GlowingMaterial_Inst_Green.M_GlowingMaterial_Inst_Green" "/Game/PostScriptum/Gameplay/Halloween/M_GlowingMaterial.M_GlowingMaterial"))))

(event Custom|TruckLoadChanged
  (bind _ju87_bomb (Variables|Default|GetJu87_Bomb))
  (bind _staticmesh (Variables|Default|GetStaticMesh))
  (Utilities|IsValid (Variables|Default|GetMyLoad)
    (:Is%20Valid
      (bind _output_get (Variables|Default|SetbCanBuild (.Filled (Default|IsCompletelyFilled (stale OnComponentBeginOverlap(Sphere) _output_get)))))
      (for _index (range 0 (- (Rendering|Material|GetNumMaterials _ju87_bomb) 1))
        (Rendering|Material|SetMaterial _ju87_bomb _index (select _output_get "/Game/PostScriptum/Gameplay/Halloween/M_GlowingMaterial_Inst_Green.M_GlowingMaterial_Inst_Green" "/Game/PostScriptum/Gameplay/Halloween/M_GlowingMaterial.M_GlowingMaterial")))
      (for _index_2 (range 0 (- (Rendering|Material|GetNumMaterials _staticmesh) 1))
        (Rendering|Material|SetMaterial _staticmesh _index_2 (select _output_get "/Game/PostScriptum/Gameplay/Halloween/M_GlowingMaterial_Inst_Green.M_GlowingMaterial_Inst_Green" "/Game/PostScriptum/Gameplay/Halloween/M_GlowingMaterial.M_GlowingMaterial"))))))

(event EventBeginPlay
  (bind _ju87_bomb (Variables|Default|GetJu87_Bomb))
  (bind _staticmesh (Variables|Default|GetStaticMesh))
  (Utilities|FlowControl|Sequence
    (:then_0
      (for _index (range 0 (- (Rendering|Material|GetNumMaterials _ju87_bomb) 1))
        (Rendering|Material|SetMaterial _ju87_bomb _index (select (stale OnComponentBeginOverlap(Sphere) _output_get_2) "/Game/PostScriptum/Gameplay/Halloween/M_GlowingMaterial_Inst_Green.M_GlowingMaterial_Inst_Green" "/Game/PostScriptum/Gameplay/Halloween/M_GlowingMaterial.M_GlowingMaterial")))
      (for _index_2 (range 0 (- (Rendering|Material|GetNumMaterials _staticmesh) 1))
        (Rendering|Material|SetMaterial _staticmesh _index_2 (select (stale OnComponentBeginOverlap(Sphere) _output_get_2) "/Game/PostScriptum/Gameplay/Halloween/M_GlowingMaterial_Inst_Green.M_GlowingMaterial_Inst_Green" "/Game/PostScriptum/Gameplay/Halloween/M_GlowingMaterial.M_GlowingMaterial"))))))

(fn ConstructionScript)

(fn TryActivating
  (params (PlayerController :type PS%20Player%20Controller%20Object%20Reference))
  (if (Variables|Default|GetbCanBuild)
    (bind _returnvalue (Game|SpawnActorfromClass "/Community_Resource_Pack/Blueprints/Z/BP_PSDeployable_Explosive_Z.BP_PSDeployable_Explosive_Z_C" (Transformation|GetActorTransform) "AlwaysSpawn" 0 (Variables|Default|GetEndGameCamera) 1 false 0))
    (Class|SQDeployable|SetTeam _returnvalue 2)
    (Default|OffLoad (Variables|Default|GetMyLoad))
    (bind _asbp_game_state_crp (Utilities|Casting|CastToBP_GameState_CRP (Game|GetGameState)))
    (Default|ToastAll _asbp_game_state_crp (Utilities|Text|MakeLiteralText "Bomb supplies have been off loaded 
Survivors gain 3 more minutes"))
    (Networking|SwitchHasAuthority
      (:Authority
        (Development|ExecuteConsoleCommand "AdminAddMatchTimeSeconds 180" 0))
      (:Remote
        _))
    (Actor|DestroyActor)
    (return true)
    (else
      (bind _asbp_ps_player_controller (Utilities|Casting|CastToBP_PS_PlayerController PlayerController))
      (Class|SQPlayerController|ClientShowToast _asbp_ps_player_controller (select (Utilities|IsValid (Variables|Default|GetMyLoad)) "Need More supplies in truck" "Supply truck needs to be closer") 5.0)
      (return false))))
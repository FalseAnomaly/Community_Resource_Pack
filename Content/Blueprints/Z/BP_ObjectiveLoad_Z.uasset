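; Truck supply-load objective for a survivor mode, counting loaded supplies against a required maximum.
; It registers itself with BP_GameState_CRP, retrying through the player controller when the game state is not yet valid.
; Count changes fire a load-changed dispatcher through RepNotify, which authority uses to toast progress and survivor time gains.
; Offloading destroys the filling meshes and silences toasts; the per-count mesh visibility logic is disconnected.
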(event Custom|ShowToastToAll
  (bind (_filled _minimumrequired _current) (CallFunction|IsCompletelyFilled))
  (if (not (Variables|Default|GetbOffLoaded))
    (bind _assqplayer_controller (Utilities|Casting|CastToSQPlayerController (Game|GetPlayerController 0)))
    (if _filled
      (if (< _minimumrequired _current)
        (Class|SQPlayerController|ShowToast _assqplayer_controller (Utilities|Text|MakeLiteralText "All Supplies have been loaded 
No time awarded for extra supplies") 5.0 false)
        (else
          (Class|SQPlayerController|ShowToast _assqplayer_controller (Utilities|Text|MakeLiteralText "All Supplies have been loaded 
Survivors gain 3 more minutes") 5.0 false)))
      (else
        (Class|SQPlayerController|ShowToast _assqplayer_controller (Utilities|Text|ToText(String) (Utilities|String|Append (Utilities|String|ToString(Integer) _current) " of " (Utilities|String|ToString(Integer) _minimumrequired) " supplies have been loaded 
Survivors gain 3 more minutes")) 5.0 false)))))

(event Custom|OnTruckLoadChanged_Event
  (CallFunction|ShowToasttoAll))

(event Custom|GameStateAvailable_Event_0
  (bind _returnvalue (Game|GetGameState))
  (Utilities|IsValid _returnvalue
    (:Is%20Valid
      (bind _asbp_game_state_crp (Utilities|Casting|CastToBP_GameState_CRP _returnvalue))
      (bind _output_get (Variables|/Community_Resource_Pack/Gameplay/Gamemodes/CRPMain/BP_GameState_CRP.BP_GameState_CRP_C|SetTruckLoadZ _asbp_game_state_crp self))
      (Default|CallOnTruckSpawned _asbp_game_state_crp _output_get))
    (:Is%20Not%20Valid
      (bind _asbp_player_controller (Utilities|Casting|CastToBP_PlayerController (Game|GetPlayerController 0)))
      (EventDispatchers|AssignGameStateAvailable _asbp_player_controller (delegate Custom|GameStateAvailable_Event_0)))))

(event EventBeginPlay
  (bind _returnvalue (Game|GetGameState))
  (|CallParentFunction)
  (Utilities|FlowControl|Sequence
    (:then_0
      (Utilities|IsValid _returnvalue
        (:Is%20Valid
          (bind _asbp_game_state_crp (Utilities|Casting|CastToBP_GameState_CRP _returnvalue))
          (bind _output_get (Variables|/Community_Resource_Pack/Gameplay/Gamemodes/CRPMain/BP_GameState_CRP.BP_GameState_CRP_C|SetTruckLoadZ _asbp_game_state_crp self))
          (Default|CallOnTruckSpawned _asbp_game_state_crp _output_get))
        (:Is%20Not%20Valid
          (bind _asbp_player_controller (Utilities|Casting|CastToBP_PlayerController (Game|GetPlayerController 0)))
          (EventDispatchers|AssignGameStateAvailable _asbp_player_controller (delegate Custom|GameStateAvailable_Event_0)))))
    (:then_1
      (Networking|SwitchHasAuthority
        (:Authority
          (EventDispatchers|BindEventtoOnTruckLoadChanged (delegate Custom|OnTruckLoadChanged_Event)))))))

(fn ConstructionScript
  (|CallParentFunction)
  (Components|Box|SetBoxExtent (Variables|Default|GetBox) (Variables|Default|GetExtent) true)
  (bind _output_get (Variables|Default|SetFillingMeshes (Utilities|Array|MakeArray (Variables|Default|GetStaticMesh1) (Variables|Default|GetStaticMesh2) (Variables|Default|GetStaticMesh3))))
  (for _array_element _output_get
    (Collision|SetCollisionEnabled _array_element "NoCollision")))

(fn AddItemtoTruck
  (Variables|Default|SetFilledAmount (+ (Variables|Default|GetFilledAmount) 1)))

(fn OnRepFilledAmount
  (if (not (Variables|Default|GetbOffLoaded))
    (Default|CallOnTruckLoadChanged)))

(fn IsCompletelyFilled
  (bind _filledamount (Variables|Default|GetFilledAmount))
  (bind _maxamount (Variables|Default|GetMaxAmount))
  (return (>= _filledamount _maxamount) _maxamount _filledamount))

(fn OffLoad
  (Variables|Default|SetbOffLoaded true))

(fn OnRepBOffLoaded
  (if (Variables|Default|GetbOffLoaded)
    (for _array_element (Variables|Default|GetFillingMeshes)
      (Components|DestroyComponent _array_element))
    (Default|CallOnTruckLoadChanged)))
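; Ammo bag pickup for the Z mode that can give a role to a player and is destroyed once loaded.
; Its sphere toggles a post-process effect for the local soldier, clearing it on death.
; Unless spawner-made, the server spawns an objective marker, removed when the role is given.
; Truck-search, progress-bar and look-check timer start-up logic is disconnected, though the cancel and cleanup handlers remain.
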(event OnComponentBeginOverlap(Sphere)
  (params (OverlappedComponent :type Primitive%20Component%20Object%20Reference) (OtherActor :type Actor%20Object%20Reference) (OtherComp :type Primitive%20Component%20Object%20Reference) (OtherBodyIndex :type Integer) (bFromSweep :type Boolean) (SweepResult :type Hit%20Result%20Structure%20%28by%20ref%29))
  (bind _asbp_mutable_soldier (Utilities|Casting|CastToBP_MutableSoldier OtherActor))
  (if (Pawn|IsLocallyControlled _asbp_mutable_soldier)
    (Variables|/Script/Engine.PostProcessComponent|SetbEnabled (Variables|Default|GetPostProcess) true)
    (EventDispatchers|AssignOnSoldierDied _asbp_mutable_soldier (delegate Custom|OnSoldierDied_Event_0))))

(event OnComponentEndOverlap(Sphere)
  (params (OverlappedComponent :type Primitive%20Component%20Object%20Reference) (OtherActor :type Actor%20Object%20Reference) (OtherComp :type Primitive%20Component%20Object%20Reference) (OtherBodyIndex :type Integer))
  (bind _asbp_mutable_soldier (Utilities|Casting|CastToBP_MutableSoldier OtherActor))
  (if (Pawn|IsLocallyControlled _asbp_mutable_soldier)
    (Variables|/Script/Engine.PostProcessComponent|SetbEnabled (Variables|Default|GetPostProcess) false)))

(event Custom|Loaded
  (Actor|DestroyActor))

(event Custom|OnSoldierDied_Event_0
  (params (DeadSoldier :type PS%20Soldier%20Object%20Reference) (Killer :type Pawn%20Object%20Reference) (DamageCauser :type Actor%20Object%20Reference) (bPointDamage :type Boolean))
  (EventDispatchers|UnbindEventfromOnSoldierDied DeadSoldier (delegate Custom|OnSoldierDied_Event_0))
  (Variables|/Script/Engine.PostProcessComponent|SetbEnabled (Variables|Default|GetPostProcess) false))

(event Custom|UpdateCheck
  (bind _usercontroller (Variables|Default|GetUserController))
  (bind _usercontroller_2 (Variables|Default|GetUserController))
  (bind _playercameramanager (Variables|/Script/Engine.PlayerController|GetPlayerCameraManager _usercontroller))
  (if (< (Math|Vector|DotProduct (Math|Vector|Normalize (- (Transformation|GetActorLocation) (Camera|GetCameraLocation _playercameramanager))) (Math|Rotator|GetRotationXVector (Camera|GetCameraRotation _playercameramanager))) 0.98)
    (Class|SQUsable|ServerStopUsed _usercontroller_2)
    (CallFunction|EndUsed _usercontroller_2)))

(event Custom|EndUsed
  (params (Controller :type Controller%20Object%20Reference))
  (bind _asplayer_controller (Utilities|Casting|CastToPlayerController Controller))
  (bind _asbp_ps_hud (Utilities|Casting|CastToBP_PS_HUD (HUD|GetHUD _asplayer_controller)))
  (Default|CancelProgressBar _asbp_ps_hud)
  (Utilities|Time|ClearandInvalidateTimerbyHandle (Variables|Default|GetUpdateCheckTimer))
  (Utilities|Time|ClearandInvalidateTimerbyHandle (Variables|Default|GetLoadingTimer))
  (Default|StopUsed (Variables|Default|GetBP_ContextSensitiveUsableComponent) _asplayer_controller))

(event Custom|LoadingTimerFinished
  (CallFunction|EndUsed (Variables|Default|GetUserController)))

(event EventBeginPlay
  (|CallParentFunction)
  (Networking|SwitchHasAuthority
    (:Authority
      (if (not (Variables|Default|GetbFromSpawner))
        (bind _returnvalue (Game|SpawnActorfromClass "/Game/PostScriptum/Gameplay/Halloween/TruckInvasion/Items/BP_HalloweenObjetiveMarkerHelper.BP_HalloweenObjetiveMarkerHelper_C" (Transformation|GetActorTransform) "AlwaysSpawn" 0 0))
        (Variables|Default|SetMarkerHelper _returnvalue)))))

(event EventGiveRoletoPlayer
  (params (player :type BP%20PS%20Mutable%20Soldier%20Object%20Reference))
  (bind _markerhelper (Variables|Default|GetMarkerHelper))
  (|CallParentFunction player)
  (Utilities|IsValid _markerhelper
    (:Is%20Valid
      (Actor|DestroyActor _markerhelper))))

(event EventEndPlay
  (params (EndPlayReason :type EEndPlayReason%20Enum :default "Destroyed"))
  (bind _usercontroller (Variables|Default|GetUserController))
  (if (Utilities|Enum|Equal(Enum) EndPlayReason "Destroyed")
    (Class|SQUsable|ServerStopUsed _usercontroller)
    (CallFunction|EndUsed _usercontroller)))

(fn ConstructionScript
  (|CallParentFunction)
  (Components|Box|SetBoxExtent (Variables|Default|GetBox) (/ (.BoxExtent (Collision|GetComponentBounds (Variables|Default|GetSkeletalMesh))) 2.0) true))

(fn FindTruck
  (params (InRadius :type Float%20%28single-precision%29))
  (bind (_outactors _returnvalue) (Collision|SphereOverlapActors (Transformation|GetActorLocation) InRadius (Utilities|Array|MakeArray "ObjectTypeQuery2" "ObjectTypeQuery1") "/Community_Resource_Pack/Blueprints/Z/BP_ObjectiveLoad_Z.BP_ObjectiveLoad_Z_C"))
  (if _returnvalue
    (bind _asbp_objective_load_z (Utilities|Casting|CastToBP_ObjectiveLoad_Z (Utilities|Array|Get(acopy) _outactors)))
    (return _asbp_objective_load_z true)
    (else
      (return 0 false))))
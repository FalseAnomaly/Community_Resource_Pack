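; Deployable ammo bag that serves only as a placement step, turning into a BP_AmmoBagPickup_Z in the world once placed.
; When not a ghost, it destroys all its primitive components on BeginPlay.
; On placement, the authority traces down against static world geometry, spawns the pickup at the hit point (or trace end) with the German deployer weapon class, then expires shortly after.
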(event EventBPonUsed
  (params (User :type Controller%20Object%20Reference)))

(event EventPlaced
  (bind _returnvalue (Transformation|GetActorLocation))
  (|CallParentFunction)
  (Networking|SwitchHasAuthority
    (:Authority
      (bind _outhit (Collision|LineTraceForObjects _returnvalue (+ _returnvalue (Math|Vector|MakeVector 0.0 0.0 -1e+03)) (Utilities|Array|MakeArray "ObjectTypeQuery1") true (Utilities|Array|MakeArray self) "None"))
      (Game|SpawnActorfromClass "/Community_Resource_Pack/Blueprints/Z/BP_AmmoBagPickup_Z.BP_AmmoBagPickup_Z_C" (Math|Transform|MakeTransform (select (.bBlockingHit (Collision|BreakHitResult _outhit)) (.ImpactPoint (Collision|BreakHitResult _outhit)) (.TraceEnd (Collision|BreakHitResult _outhit)))) "AlwaysSpawn" 0 false "/Game/PostScriptum/Gameplay/Halloween/TruckInvasion/Items/BP_AmmoBag_Deployer_GER_H.BP_AmmoBag_Deployer_GER_H_C" true true 0)
      (Actor|SetLifeSpan 1.1))))

(event EventBeginPlay
  (|CallParentFunction)
  (if (not (Class|SQDeployable|IsGhost))
    (for _array_element (Actor|GetComponentsByClass "/Script/Engine.PrimitiveComponent")
      (Components|DestroyComponent _array_element))))

(fn ConstructionScript
  (|CallParentFunction))
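; End-of-match victory scene actor for the Z mode, showing either the zombie or human victory display alongside match stats.
; Init puts the end-of-match stats widget on screen and hides all pawns, soldiers, projectiles and destroyed vehicles.
; The winning team selects the class of the WinnerTeamDisplay child actor.
; The local player's view switches to this actor, which registers itself with the player camera manager.
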(event EventBeginPlay)

(event Collision|EventActorBeginOverlap
  (params (OtherActor :type Actor%20Object%20Reference)))

(event EventTick
  (params (DeltaSeconds :type Float%20%28single-precision%29)))

(event EventInit
  (params (WinnerTeam :type Byte :default 0) (Team1Stats :type Processed%20Stats%20Container%20Structure) (Team2Stats :type Processed%20Stats%20Container%20Structure))
  (bind _returnvalue (Game|GetPlayerController 0))
  (bind _returnvalue_2 (Class|SQTeamInterface|GetTeamId(Message) _returnvalue))
  (Variables|Default|SetMyTeam (Math|Conversions|ToByte(Integer) _returnvalue_2))
  (Utilities|FlowControl|Sequence
    (:then_0
      (bind _returnvalue_3 (CallFunction|CreateVictoryStatsWidget _returnvalue Team2Stats Team1Stats WinnerTeam))
      (bind _output_get (Variables|Default|SetMyStatsScreen _returnvalue_3))
      (UserInterface|Viewport|AddtoViewport _output_get 0)
      (Utilities|FlowControl|Sequence
        (:then_0
          (bind _outactors (Actor|GetAllActorsOfClass "/Game/PostScriptum/Blueprints/BP_PS_DestroyedVehicle.BP_PS_DestroyedVehicle_C"))
          (for _array_element _outactors
            (Class|SQBlueprintLibrary|SetActorHiddeninGame _array_element true true)))
        (:then_1
          (bind _outactors_2 (Actor|GetAllActorsOfClass "/Script/Squad.SQPawn"))
          (for _array_element_2 _outactors_2
            (Class|SQBlueprintLibrary|SetActorHiddeninGame _array_element_2 true true)))
        (:then_2
          (bind _outactors_3 (Actor|GetAllActorsOfClass "/Script/Squad.SQSoldier"))
          (for _array_element_3 _outactors_3
            (Class|SQBlueprintLibrary|SetActorHiddeninGame _array_element_3 true true)))
        (:then_3
          (bind _outactors_4 (Actor|GetAllActorsOfClass "/Script/Squad.SQProjectile"))
          (for _array_element_4 _outactors_4
            (Class|SQBlueprintLibrary|SetActorHiddeninGame _array_element_4 true true)))))
    (:then_1
      (bind _output_get_2 (Variables|Default|SetWinnerTeam WinnerTeam))
      (ChildActorComponent|SetChildActorClass (Variables|Default|GetWinnerTeamDisplay) (Utilities|Select :Index _output_get_2 :Option%200 0 :Option%201 (Variables|Default|GetZombieVictoryDisplayClass) :Option%202 (Variables|Default|GetHumanVictoryDisplayClass))))
    (:then_3
      (Game|Player|SetViewTargetwithBlend (Game|GetPlayerController 0) self 0.0 "VTBlend_Linear" 0.0 false))
    (:then_4
      (bind _asbp_psplayer_camera_manager (Utilities|Casting|CastToBP_PSPlayerCameraManager (Game|GetPlayerCameraManager 0)))
      (Variables|/Game/PostScriptum/Blueprints/BP_PSPlayerCameraManager.BP_PSPlayerCameraManager_C|SetVictoryDisplay _asbp_psplayer_camera_manager self))))

(fn ConstructionScript
  (|CallParentFunction))

(fn CreateVictoryStatsWidget
  (params (OwningPlayer :type Player%20Controller%20Object%20Reference) (Team2Stats :type Processed%20Stats%20Container%20Structure) (Team1Stats :type Processed%20Stats%20Container%20Structure) (WinnerTeam :type Byte :default 0))
  (bind _returnvalue (UserInterface|CreateWidget "/Community_Resource_Pack/UI/UMG_PS_EndOfMatchStats_Z.UMG_PS_EndOfMatchStats_Z_C" OwningPlayer Team2Stats Team1Stats WinnerTeam))
  (return _returnvalue))
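; Victory display actor for a faction, which shows soldier meshes matching a given team's roles.
; Init reads the team info's class default object and calls CopyMeshFrom once for the default commander role and twice for the default role.
; CopyMeshFrom takes the skeletal mesh from the role's soldier class default object and applies it to a target mesh, so no soldier needs spawning.
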(event Custom|Init
  (params (TeamInfo :type SQ%20Team%20Info%20Class%20Reference))
  (bind _returnvalue (Class|SQBlueprintLibrary|GetDefaultObjectfor TeamInfo))
  (bind _asbp_ps_team_info (Utilities|Casting|CastToBP_PS_TeamInfo _returnvalue))
  (CallFunction|CopyMeshfrom (Variables|/Script/PostScriptum.PSTeamInfo|GetDefaultCommanderRole _asbp_ps_team_info))
  (CallFunction|CopyMeshfrom (Variables|/Script/Squad.SQTeamInfo|GetDefaultRole _asbp_ps_team_info))
  (CallFunction|CopyMeshfrom (Variables|/Script/Squad.SQTeamInfo|GetDefaultRole _asbp_ps_team_info)))

(event EventBeginPlay)

(event Collision|EventActorBeginOverlap
  (params (OtherActor :type Actor%20Object%20Reference)))

(event EventTick
  (params (DeltaSeconds :type Float%20%28single-precision%29)))

(fn ConstructionScript)

(fn CopyMeshfrom
  (params (role :type SQ%20Role%20Settings%20Object%20Reference) (TargetMesh :type Skinned%20Mesh%20Component%20Object%20Reference))
  (bind _returnvalue (Class|SQBlueprintLibrary|GetDefaultObjectfor (Variables|/Script/Squad.SQRoleSettings|GetSoldierClass role)))
  (bind _aspssoldier (Utilities|Casting|CastToPSSoldier _returnvalue))
  (Class|SkinnedMeshComponent|SetSkeletalMesh TargetMesh (Variables|/Script/Engine.SkinnedMeshComponent|GetSkeletalMesh (Variables|/Script/Engine.Character|GetMesh _aspssoldier)) true))
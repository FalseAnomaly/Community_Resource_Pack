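; Objective spawner that places an ammo bag pickup for the objective when activated.
; Activate spawns the pickup at SpawnPoint, binds to its destruction and marks the spawner active.
; While inactive, a server-side sphere overlap by a soldier on the human team destroys the spawner.
; A PickupGrabbed event also destroys it, apparently once the spawned pickup is gone.
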(event OnComponentBeginOverlap(OverlapSphere)
  (params (OverlappedComponent :type Primitive%20Component%20Object%20Reference) (OtherActor :type Actor%20Object%20Reference) (OtherComp :type Primitive%20Component%20Object%20Reference) (OtherBodyIndex :type Integer) (bFromSweep :type Boolean) (SweepResult :type Hit%20Result%20Structure%20%28by%20ref%29))
  (Networking|SwitchHasAuthority
    (:Authority
      (if (not (Variables|Default|GetbIsActivated))
        (bind _asbp_mutable_soldier (Utilities|Casting|CastToBP_MutableSoldier OtherActor))
        (bind _returnvalue (Class|SQTeamInterface|GetTeamId(Message) (Pawn|GetController _asbp_mutable_soldier)))
        (if (== (Variables|Default|GetHumanTeamID) _returnvalue)
          (Actor|DestroyActor))))))

(event Custom|PickupGrabbed
  (params (pickupActor :type Actor%20Object%20Reference))
  (Actor|DestroyActor))

(event EventTick
  (params (DeltaSeconds :type Float%20%28single-precision%29)))

(fn ConstructionScript)

(fn Activate
  (bind _returnvalue (Game|SpawnActorfromClass "/Community_Resource_Pack/Blueprints/Z/BP_AmmoBagPickup_Z.BP_AmmoBagPickup_Z_C" (Class|SQBlueprintLibrary|GetComponentTransform (Variables|Default|GetSpawnPoint)) "AlwaysSpawn" 0 true "/Community_Resource_Pack/Blueprints/Z/BP_AmmoBag_Deployer_Z.BP_AmmoBag_Deployer_Z_C" true true 0))
  (bind _output_get (LocalVariables|SetMyItem _returnvalue))
  (Game|BindEventtoOnDestroyed _output_get (EventDispatchers|CreateEvent :!event Custom|PickupGrabbed))
  (Variables|Default|SetbIsActivated true))
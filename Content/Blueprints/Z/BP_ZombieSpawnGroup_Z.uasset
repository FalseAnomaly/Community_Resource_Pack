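; Zombie spawn group that tracks enemy-team humans inside its radius and flags HumanNearby while any are present.
; On the authority, radius overlaps add or remove soldiers, including seated vehicle occupants, and death events also remove tracked soldiers.
; When the list empties, a timer clears the flag after ReactivationTime; a new qualifying entry cancels it.
; Older team-neutral and SpawningEnabled toggling remains as unreachable nodes.
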(event OnComponentBeginOverlap(Radius)
  (params (OverlappedComponent :type Primitive%20Component%20Object%20Reference) (OtherActor :type Actor%20Object%20Reference) (OtherComp :type Primitive%20Component%20Object%20Reference) (OtherBodyIndex :type Integer) (bFromSweep :type Boolean) (SweepResult :type Hit%20Result%20Structure%20%28by%20ref%29))
  (Networking|SwitchHasAuthority
    (:Authority
      (bind _asbp_ps_soldier_z (Utilities|Casting|CastToBP_PS_Soldier_Z OtherActor)
        (:then
          (if (and (not (Variables|/Community_Resource_Pack/Soldiers/Z/BP_PS_Soldier_Z.BP_PS_Soldier_Z_C|GetbIsZombie _asbp_ps_soldier_z)) (== (Variables|Default|GetEnemyTeam) (Class|SQSoldier|GetTeam _asbp_ps_soldier_z)))
            (Utilities|Array|AddUnique (Variables|Default|GetActiveEnemies) _asbp_ps_soldier_z)
            (EventDispatchers|BindEventtoOnSoldierDied _asbp_ps_soldier_z (delegate Custom|OnSoldierDied))
            (Utilities|Time|ClearandInvalidateTimerbyHandle (Variables|Default|GetReactivationTimer))
            (Variables|Default|SetHumanNearby true)))
        (:CastFailed
          (bind _assqvehicle (Utilities|Casting|CastToSQVehicle OtherActor))
          (for _array_element (Class|SQVehicle|GetSeats _assqvehicle)
            (Utilities|IsValid (Variables|/Script/Squad.SQVehicleSeatComponent|GetSeatedPlayer _array_element)
              (:Is%20Valid
                (bind _asbp_ps_soldier_z_2 (Utilities|Casting|CastToBP_PS_Soldier_Z (Class|SQPlayerState|GetSoldier (Variables|/Script/Squad.SQVehicleSeatComponent|GetSeatedPlayer _array_element))))
                (if (and (not (Variables|/Community_Resource_Pack/Soldiers/Z/BP_PS_Soldier_Z.BP_PS_Soldier_Z_C|GetbIsZombie _asbp_ps_soldier_z_2)) (== (Variables|Default|GetEnemyTeam) (Class|SQSoldier|GetTeam _asbp_ps_soldier_z_2)))
                  (Utilities|Array|AddUnique (Variables|Default|GetActiveEnemies) _asbp_ps_soldier_z_2)
                  (EventDispatchers|BindEventtoOnSoldierDied _asbp_ps_soldier_z_2 (delegate Custom|OnSoldierDied))
                  (Utilities|Time|ClearandInvalidateTimerbyHandle (Variables|Default|GetReactivationTimer))
                  (Variables|Default|SetHumanNearby true))))))))))

(event OnComponentEndOverlap(Radius)
  (params (OverlappedComponent :type Primitive%20Component%20Object%20Reference) (OtherActor :type Actor%20Object%20Reference) (OtherComp :type Primitive%20Component%20Object%20Reference) (OtherBodyIndex :type Integer))
  (Networking|SwitchHasAuthority
    (:Authority
      (bind _asbp_ps_soldier_z (Utilities|Casting|CastToBP_PS_Soldier_Z OtherActor)
        (:then
          (if (not (Variables|/Community_Resource_Pack/Soldiers/Z/BP_PS_Soldier_Z.BP_PS_Soldier_Z_C|GetbIsZombie _asbp_ps_soldier_z))
            (CallFunction|CheckifClearOfEnemies _asbp_ps_soldier_z)))
        (:CastFailed
          (bind _assqvehicle (Utilities|Casting|CastToSQVehicle OtherActor))
          (for _array_element (Class|SQVehicle|GetSeats _assqvehicle)
            (Utilities|IsValid (Variables|/Script/Squad.SQVehicleSeatComponent|GetSeatedPlayer _array_element)
              (:Is%20Valid
                (bind _asbp_ps_soldier_z_2 (Utilities|Casting|CastToBP_PS_Soldier_Z (Class|SQPlayerState|GetSoldier (Variables|/Script/Squad.SQVehicleSeatComponent|GetSeatedPlayer _array_element))))
                (if (not (Variables|/Community_Resource_Pack/Soldiers/Z/BP_PS_Soldier_Z.BP_PS_Soldier_Z_C|GetbIsZombie _asbp_ps_soldier_z_2))
                  (CallFunction|CheckifClearOfEnemies _asbp_ps_soldier_z_2))))))))))

(event Custom|OnSoldierDied
  (params (DeadSoldier :type PS%20Soldier%20Object%20Reference) (Killer :type Pawn%20Object%20Reference) (DamageCauser :type Actor%20Object%20Reference) (bPointDamage :type Boolean))
  (CallFunction|CheckifClearOfEnemies DeadSoldier))

(event Custom|CheckIfClearOfEnemies
  (params (LastLeavingSoldier :type PS%20Soldier%20Object%20Reference))
  (bind _activeenemies (Variables|Default|GetActiveEnemies))
  (Utilities|Array|RemoveItem _activeenemies LastLeavingSoldier)
  (if (== (Utilities|Array|Length _activeenemies) 0)
    (bind _returnvalue (Utilities|Time|SetTimerbyEvent (delegate Custom|ReactivateSpawn) (Variables|Default|GetReactivationTime)))
    (Variables|Default|SetReactivationTimer _returnvalue)))

(event Custom|ReactivateSpawn
  (Variables|Default|SetHumanNearby false))

(event EventBeginPlay
  (|CallParentFunction)
  (Networking|SwitchHasAuthority
    (:Authority
      (Class|SQGameSpawn|SetTeam (Variables|Default|GetDefaultTeam)))))

(fn ConstructionScript
  (|CallParentFunction))
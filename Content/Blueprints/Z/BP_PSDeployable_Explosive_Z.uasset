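; Deployable bomb objective that one team builds, arms and protects while the enemy team tries to destroy it.
; An authority timer polls Health until fully built, then announces it; activation then sets BombActive, whose RepNotify starts fuse effects, objective UI and team toasts.
; Tick counts down to an end-game camera, explosion and forced match end for team 2, while depleting BombHealth through damage ends it for team 1.
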(event Custom|ActivateBomb
  (Variables|Default|SetbBombActive true))

(event Custom|SwitchToEndGameCamera
  (bind _returnvalue (Game|GetPlayerController 0))
  (if (Pawn|IsLocalPlayerController _returnvalue)
    (bind _output_get (Variables|Default|SetLocalPC _returnvalue))
    (Input|SetIgnoreMoveInput _output_get true)
    (for _array_element (Variables|/Script/Engine.GameStateBase|GetPlayerArray (Game|GetGameState))
      (bind _aspsplayer_state (Utilities|Casting|CastToPSPlayerState _array_element))
      (Rendering|SetActorHiddenInGame (Class|SQPlayerState|GetSoldier _aspsplayer_state) true))
    (Game|Player|SetViewTargetwithBlend (Variables|Default|GetLocalPC) (Variables|Default|GetEndGameCamera) 0.0 "VTBlend_Linear" 0.0 false)
    (Audio|Components|Audio|Stop (Variables|Default|GetSFX_Fuse))))

(event Custom|OnFinishedBomb
  (bind _assqplayer_controller (Utilities|Casting|CastToSQPlayerController (Game|GetPlayerController 0)))
  (Class|SQPlayerController|ShowToast _assqplayer_controller (Utilities|Select :Index (Class|SQPlayerController|GetTeam _assqplayer_controller) :Option%200 "" :Option%201 (Utilities|Text|MakeLiteralText "Enemy has Built the bomb. Stop them") :Option%202 (Utilities|Text|MakeLiteralText "Bomb has been built. Activate it")) 4.0 false)
  (bind _asbp_game_state_crp (Utilities|Casting|CastToBP_GameState_CRP (Game|GetGameState)))
  (Default|SignalImportantEvent _asbp_game_state_crp 1.0))

(event Custom|StateCheck
  (if (== (Variables|Default|GetHealth) (Variables|Default|GetMaxHealth))
    (Utilities|Time|ClearandInvalidateTimerbyHandle (Variables|Default|GetStateCheckTimerHandle))
    (CallFunction|OnFinishedBomb)))

(event Game|Damage|EventAnyDamage
  (params (Damage :type Float%20%28single-precision%29) (DamageType :type Damage%20Type%20Object%20Reference) (InstigatedBy :type Controller%20Object%20Reference) (DamageCauser :type Actor%20Object%20Reference))
  (|CallParentFunction Damage DamageType InstigatedBy DamageCauser)
  (bind _output_get (Variables|Default|SetBombHealth (- (Variables|Default|GetBombHealth) Damage)))
  (if (<= _output_get 0.0)
    (bind _asbp_game_mode (Utilities|Casting|CastToBP_GameMode (Game|GetGameMode)))
    (Default|ForceEndMatch _asbp_game_mode 1)
    (Utilities|FlowControl|Delay 1.0)
    (Actor|DestroyActor)))

(event EventTick
  (params (DeltaSeconds :type Float%20%28single-precision%29))
  (|CallParentFunction DeltaSeconds)
  (Utilities|FlowControl|Sequence
    (:then_0
      (if (and (> (Variables|Default|GetBombTimer) 0.0) (Variables|Default|GetbBombActive))
        (bind _output_get (Variables|Default|SetBombTimer (- (Variables|Default|GetBombTimer) DeltaSeconds)))
        (Networking|SwitchHasAuthority
          (:Authority
            (if (<= _output_get 0.0)
              (CallFunction|SwitchtoEndGameCamera)
              (Utilities|FlowControl|Delay 1.0)
              (Game|SpawnActorfromClass "/Game/PostScriptum/Gameplay/Halloween/TruckInvasion/Items/BP_BombExplosion.BP_BombExplosion_C" (Transformation|GetActorTransform) "AlwaysSpawn" 0 0)
              (Class|SQBlueprintLibrary|SetActorHiddeninGame self true true)
              (Utilities|FlowControl|Delay 1e+01)
              (bind _asbp_game_mode (Utilities|Casting|CastToBP_GameMode (Game|GetGameMode)))
              (Default|ForceEndMatch _asbp_game_mode 2))))))))

(event EventBPonUsed
  (params (User :type Controller%20Object%20Reference))
  (if (not (Variables|Default|GetbBombActive))
    (Default|Used (Variables|Default|GetBP_ContextSensitiveUsableComponent) User)))

(event EventOnActivated
  (params (ActivatedBy :type Player%20Controller%20Object%20Reference))
  (Networking|SwitchHasAuthority
    (:Authority
      (if (== (Variables|Default|GetHealth) (Variables|Default|GetMaxHealth))
        (if (not (Variables|Default|GetbBombActive))
          (CallFunction|ActivateBomb)
          (bind _asbp_game_state_crp (Utilities|Casting|CastToBP_GameState_CRP (Game|GetGameState)))
          (Default|SignalImportantEvent _asbp_game_state_crp 1.0))
        (else
          (bind _asbp_ps_player_controller (Utilities|Casting|CastToBP_PS_PlayerController ActivatedBy))
          (Default|ClientNotification _asbp_ps_player_controller "Bomb not completely built" "Negative"))))))

(event EventBPStopUsed
  (params (User :type Controller%20Object%20Reference))
  (Default|StopUsed (Variables|Default|GetBP_ContextSensitiveUsableComponent) User))

(event EventBeginPlay
  (|CallParentFunction)
  (Networking|SwitchHasAuthority
    (:Authority
      (bind _returnvalue (Utilities|Time|SetTimerbyEvent (delegate Custom|StateCheck) 1.0 true))
      (Variables|Default|SetStateCheckTimerHandle _returnvalue))))

(fn ConstructionScript
  (|CallParentFunction))

(fn OnRepBBombActive
  (if (Variables|Default|GetbBombActive)
    (Actor|Tick|SetActorTickEnabled true)
    (Networking|CanExecuteCosmeticEvents
      (:True
        (Components|Activation|Activate (Variables|Default|GetSFX_Fuse) false)
        (Rendering|SetVisibility (Variables|Default|GetBomb_Sparks) true false)
        (bind _asbp_game_state_crp (Utilities|Casting|CastToBP_GameState_CRP (Game|GetGameState)))
        (Default|BombActivated (Variables|/PSCommunityResourcePack/Gameplay/Gamemodes/CRPMain/BP_GameState_CRP.BP_GameState_CRP_C|GetObjectiveStateWidgetZ _asbp_game_state_crp) self)
        (bind _asbp_ps_player_controller (Utilities|Casting|CastToBP_PS_PlayerController (Widget|GetOwningPlayer (Variables|/PSCommunityResourcePack/Gameplay/Gamemodes/CRPMain/BP_GameState_CRP.BP_GameState_CRP_C|GetObjectiveStateWidgetZ _asbp_game_state_crp))))
        (Class|SQPlayerController|ClientShowToast _asbp_ps_player_controller (Utilities|Text|ToText(String) (Utilities|String|Append "Bomb has been armed," (Utilities|Select :Index (Class|SQPlayerController|GetTeam _asbp_ps_player_controller) :Option%200 "" :Option%201 "Destroy it before " :Option%202 "Protect it for ") (Utilities|String|LeftChop (Class|KismetStringLibrary|TimeSecondstoString (Variables|Default|GetBombTimer)) 3))) 5.0)))))

(fn OnRepBombTimer)

(fn DoDamageFX
  (bind _returnvalue (Transformation|GetActorLocation))
  (Audio|SpawnSoundatLocation "/Game/Audio/Impacts/Bullethits/Wood/Wood_solid/Small/bhit_small_wood_Cue.bhit_small_wood_Cue" _returnvalue "0, 0, 0" 1.0 1.0 0.0 0 0)
  (Effects|SpawnEmitteratLocation "/Game/Particles/Impacts/Auto_Cannons/30mm_AP/bhit_30mm_AP_wood.bhit_30mm_AP_wood" _returnvalue))